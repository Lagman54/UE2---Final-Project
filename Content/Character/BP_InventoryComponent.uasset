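; Player inventory component holding a ten-slot item array shown through WBP_Inventory, which refreshes after every change.
; Adding merges stackable items by name or fills the first "None" slot; dropping spawns a BP_Item at the player unless undroppable.
; Using a key, shotgun shelf or medallion item calls Unlock on the hero's current unlockable.
; Opening the inventory locks movement and aiming, unless that unlockable restricts it.
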(event Custom|UseItem_Event
  (params (Item%20Index :type Integer))
  (bind _items (Variables|Default|GetItems))
  (bind _output (Utilities|Array|Get(acopy) _items Item%20Index))
  (bind (_name _stackable _quantity _thumbnail _mesh _meshscale _collisionscale _key_ _shotgunshelf_ _undroppable_ _medalion_) (Utilities|Struct|BreakS_ItemStructure _output))
  (bind _returnvalue (Utilities|String|ToString(Text) _name))
  (Development|PrintString "Use item")
  (if _key_
    (bind _asbp_hero (Utilities|Casting|CastToBP_Hero (Game|GetPlayerCharacter 0)))
    (bind _result (Default|Unlock (Variables|/Game/Character/BP_Hero.BP_Hero_C|GetCurrentUnlockable _asbp_hero) (Utilities|String|ToString(Text) _name)))
    (if (not _result)
      (Development|PrintString "Wrong key"))
    (elif _shotgunshelf_
      (bind _asbp_hero_2 (Utilities|Casting|CastToBP_Hero (Game|GetPlayerCharacter 0)))
      (Default|Unlock (Variables|/Game/Character/BP_Hero.BP_Hero_C|GetCurrentUnlockable _asbp_hero_2) _returnvalue)
      (elif _medalion_
        (bind _asbp_hero_3 (Utilities|Casting|CastToBP_Hero (Game|GetPlayerCharacter 0)))
        (Default|Unlock (Variables|/Game/Character/BP_Hero.BP_Hero_C|GetCurrentUnlockable _asbp_hero_3) _returnvalue)))))

(event Custom|Add%20Item
  (params (Item :type BP%20Item%20Object%20Reference))
  (bind _inventorywidget (Variables|Default|GetInventoryWidget))
  (bind (_name _stackable _quantity) (Utilities|Struct|BreakS_ItemStructure (Variables|/Game/Blueprints/Inventory/BP_Item.BP_Item_C|GetItem Item)))
  ;[0.15 0.15 0.15 0.5] Add Item
  (Variables|Default|SetItemNotFound true)
  (for (_array_element _array_index) (Variables|Default|GetItems)
    (Utilities|IsValid Item
      (:Is%20Valid
        (if (Math|Boolean|ANDBoolean (Utilities|Enum|Equal(Enum) (.Name (Utilities|Struct|BreakS_ItemStructure _array_element)) _name) _stackable (.Stackable (Utilities|Struct|BreakS_ItemStructure _array_element)))
          (Utilities|Array|SetArrayElem (Variables|Default|GetItems) _array_index (Utilities|Struct|MakeS_ItemStructure (.Name (Utilities|Struct|BreakS_ItemStructure _array_element)) (.Stackable (Utilities|Struct|BreakS_ItemStructure _array_element)) (+ (.Quantity (Utilities|Struct|BreakS_ItemStructure _array_element)) _quantity) (.Thumbnail (Utilities|Struct|BreakS_ItemStructure _array_element)) (.Mesh (Utilities|Struct|BreakS_ItemStructure _array_element))))
          (Default|LoadInventory _inventorywidget self)
          (Variables|Default|SetItemNotFound false)
          (Actor|DestroyActor Item)))))
  (if (Variables|Default|GetItemNotFound)
    (bind (_array_element_2 _array_index_2) (Utilities|Array|ForEachLoopwithBreak (Variables|Default|GetItems) :!label _label)
      (:LoopBody
        (Utilities|IsValid Item
          (:Is%20Valid
            (if (Utilities|Enum|Equal(Enum) (.Name (Utilities|Struct|BreakS_ItemStructure _array_element_2)) (Utilities|Text|MakeLiteralText "None"))
              (Utilities|Array|SetArrayElem (Variables|Default|GetItems) _array_index_2 (Variables|/Game/Blueprints/Inventory/BP_Item.BP_Item_C|GetItem Item))
              (Default|LoadInventory _inventorywidget self)
              (Actor|DestroyActor Item)
              (goto _label Break))))))))

(event Custom|DropItem_Event
  (params (ItemIndex :type Integer))
  (bind _items (Variables|Default|GetItems))
  (bind _output (Utilities|Array|Get(acopy) _items ItemIndex))
  ;[0.15 0.15 0.15 0.5] Drop Item
  (if (.Undroppable? (Utilities|Struct|BreakS_ItemStructure _output))
    (Development|PrintString "you cant drop this item" true true "(R=0.000000,G=0.660000,B=1.000000,A=1.000000)" 4.0)
    (else
      (Game|SpawnActorfromClass "/Game/Blueprints/Inventory/BP_Item.BP_Item_C" (Transformation|GetActorTransform (Game|GetPlayerCharacter 0)) "Undefined" "MultiplyWithRoot" 0 _output 0)
      (Utilities|Array|SetArrayElem :TargetArray (Variables|Default|GetItems) :Index ItemIndex)
      (Default|LoadInventory (Variables|Default|GetInventoryWidget) self))))

(event Custom|Force%20Close%20Inventory
  (bind _returnvalue (Game|GetPlayerController 0))
  (bind _inventorywidget (Variables|Default|GetInventoryWidget))
  (bind _character (Variables|Default|GetCharacter))
  (bind _currentcontextmenu (Variables|/Game/Blueprints/Inventory/Widgets/WBP_Inventory.WBP_Inventory_C|GetCurrentContextMenu _inventorywidget))
  ;[0.15 0.15 0.15 0.5] Open Inventory
  (Widget|RemovefromParent (Variables|Default|GetInventoryWidget))
  (Input|SetInputModeGameOnly _returnvalue false)
  (Variables|/Script/Engine.PlayerController|SetbShowMouseCursor _returnvalue false)
  (Variables|/Game/Character/BP_Hero.BP_Hero_C|SetAimingAllowed _character true)
  (Default|UnlockCharacter _character)
  (Utilities|IsValid _currentcontextmenu
    (:Is%20Valid
      (Widget|RemovefromParent _currentcontextmenu))))

(event Custom|Add%20ItemS
  (params (ItemS :type S%20Item%20Structure%20Structure))
  (bind (_name _stackable _quantity) (Utilities|Struct|BreakS_ItemStructure ItemS))
  (bind _inventorywidget (Variables|Default|GetInventoryWidget))
  (Variables|Default|SetItemNotFound true)
  (for (_array_element _array_index) (Variables|Default|GetItems)
    (if (Math|Boolean|ANDBoolean (Utilities|Enum|Equal(Enum) (.Name (Utilities|Struct|BreakS_ItemStructure _array_element)) _name) _stackable (.Stackable (Utilities|Struct|BreakS_ItemStructure _array_element)))
      (Utilities|Array|SetArrayElem (Variables|Default|GetItems) _array_index (Utilities|Struct|MakeS_ItemStructure (.Name (Utilities|Struct|BreakS_ItemStructure _array_element)) (.Stackable (Utilities|Struct|BreakS_ItemStructure _array_element)) (+ (.Quantity (Utilities|Struct|BreakS_ItemStructure _array_element)) _quantity) (.Thumbnail (Utilities|Struct|BreakS_ItemStructure _array_element)) (.Mesh (Utilities|Struct|BreakS_ItemStructure _array_element))))
      (Default|LoadInventory _inventorywidget self)
      (Variables|Default|SetItemNotFound false)))
  (if (Variables|Default|GetItemNotFound)
    (bind (_array_element_2 _array_index_2) (Utilities|Array|ForEachLoopwithBreak (Variables|Default|GetItems) :!label _label)
      (:LoopBody
        (if (Utilities|Enum|Equal(Enum) (.Name (Utilities|Struct|BreakS_ItemStructure _array_element_2)) (Utilities|Text|MakeLiteralText "None"))
          (Utilities|Array|SetArrayElem (Variables|Default|GetItems) _array_index_2 ItemS)
          (Default|LoadInventory _inventorywidget self)
          (goto _label Break))))))

(event Custom|Delete%20Item%20By%20Index
  (params (Item%20Index :type Integer))
  (Utilities|Array|SetArrayElem :TargetArray (Variables|Default|GetItems) :Index Item%20Index)
  (Default|LoadInventory (Variables|Default|GetInventoryWidget) self))

(event Custom|Delete%20Item%20By%20Name
  (params (Name :type Text))
  (bind (_array_element _array_index) (Utilities|Array|ForEachLoopwithBreak (Variables|Default|GetItems) :!label _label)
    (:LoopBody
      (if (Utilities|Enum|Equal(Enum) (.Name (Utilities|Struct|BreakS_ItemStructure _array_element)) Name)
        (Utilities|Array|SetArrayElem :TargetArray (Variables|Default|GetItems) :Index _array_index)
        (goto _label Break)))
    (:Completed
      (Default|LoadInventory (Variables|Default|GetInventoryWidget) self))))

(event Custom|Force%20open%20inventory
  (bind _returnvalue (Game|GetPlayerController 0))
  (bind _returnvalue_2 (Game|GetPlayerController 0))
  (bind _inventorywidget (Variables|Default|GetInventoryWidget))
  (bind _inventorywidget_2 (Variables|Default|GetInventoryWidget))
  (bind _character (Variables|Default|GetCharacter))
  (bind _character_2 (Variables|Default|GetCharacter))
  (bind _character_3 (Variables|Default|GetCharacter))
  (bind _currentcontextmenu (Variables|/Game/Blueprints/Inventory/Widgets/WBP_Inventory.WBP_Inventory_C|GetCurrentContextMenu _inventorywidget_2))
  (bind _currentunlockable (Variables|/Game/Character/BP_Hero.BP_Hero_C|GetCurrentUnlockable _character))
  ;[0.15 0.15 0.15 0.5] Open Inventory
  (if (Widget|IsVisible (Variables|Default|GetInventoryWidget))
    (Widget|RemovefromParent _inventorywidget)
    (Input|SetInputModeGameOnly _returnvalue false)
    (Variables|/Script/Engine.PlayerController|SetbShowMouseCursor _returnvalue false)
    (Variables|/Game/Character/BP_Hero.BP_Hero_C|SetAimingAllowed _character_2 true)
    (Default|UnlockCharacter _character_2)
    (Utilities|IsValid _currentcontextmenu
      (:Is%20Valid
        (Widget|RemovefromParent _currentcontextmenu)))
    (elif (Utilities|IsValidInterface _currentunlockable)
      (bind _result (Default|InventoryRestricted? _currentunlockable))
      (if (not _result)
        (Input|SetInputModeGameandUI _returnvalue_2 _inventorywidget "DoNotLock" true false :!label _label)
        (UserInterface|Viewport|AddtoViewport _inventorywidget 0)
        (Variables|/Script/Engine.PlayerController|SetbShowMouseCursor _returnvalue_2 true)
        (Variables|/Game/Character/BP_Hero.BP_Hero_C|SetAimingAllowed _character_3 false)
        (Default|LockCharacter _character_3))
      (else
        (goto _label)))))

(event Input|EnhancedActionEvents|EnhancedInputActionIA_OpenInventory
  (params (ActionValue :type Boolean) (ElapsedSeconds :type Float%20%28double-precision%29) (TriggeredSeconds :type Float%20%28double-precision%29) (InputAction :type Input%20Action%20Object%20Reference :default "/Game/Character/Input/IA_OpenInventory.IA_OpenInventory"))
  (bind _returnvalue (Game|GetPlayerController 0))
  (bind _returnvalue_2 (Game|GetPlayerController 0))
  (bind _inventorywidget (Variables|Default|GetInventoryWidget))
  (bind _inventorywidget_2 (Variables|Default|GetInventoryWidget))
  (bind _character (Variables|Default|GetCharacter))
  (bind _character_2 (Variables|Default|GetCharacter))
  (bind _character_3 (Variables|Default|GetCharacter))
  (bind _currentcontextmenu (Variables|/Game/Blueprints/Inventory/Widgets/WBP_Inventory.WBP_Inventory_C|GetCurrentContextMenu _inventorywidget_2))
  (bind _currentunlockable (Variables|/Game/Character/BP_Hero.BP_Hero_C|GetCurrentUnlockable _character))
  ;[0.15 0.15 0.15 0.5] Open Inventory
  (:Started
    (if (Widget|IsVisible (Variables|Default|GetInventoryWidget))
      (Widget|RemovefromParent _inventorywidget)
      (Input|SetInputModeGameOnly _returnvalue false)
      (Variables|/Script/Engine.PlayerController|SetbShowMouseCursor _returnvalue false)
      (Variables|/Game/Character/BP_Hero.BP_Hero_C|SetAimingAllowed _character_2 true)
      (Default|UnlockCharacter _character_2)
      (Utilities|IsValid _currentcontextmenu
        (:Is%20Valid
          (Widget|RemovefromParent _currentcontextmenu)))
      (elif (Utilities|IsValidInterface _currentunlockable)
        (bind _result (Default|InventoryRestricted? _currentunlockable))
        (if (not _result)
          (Input|SetInputModeGameandUI _returnvalue_2 _inventorywidget "DoNotLock" true false :!label _label)
          (UserInterface|Viewport|AddtoViewport _inventorywidget 0)
          (Variables|/Script/Engine.PlayerController|SetbShowMouseCursor _returnvalue_2 true)
          (Variables|/Game/Character/BP_Hero.BP_Hero_C|SetAimingAllowed _character_3 false)
          (Default|LockCharacter _character_3))
        (else
          (goto _label))))))

(event EventBeginPlay
  (bind _returnvalue (UserInterface|CreateWidget "/Game/Blueprints/Inventory/Widgets/WBP_Inventory.WBP_Inventory_C"))
  (Variables|Default|SetInventoryWidget _returnvalue)
  (Utilities|Array|Resize (Variables|Default|GetItems) 10)
  (Default|LoadInventory (Variables|Default|GetInventoryWidget) self)
  (EventDispatchers|AssignDropItem (Variables|Default|GetInventoryWidget) (delegate Custom|DropItem_Event))
  (bind _asbp_hero (Utilities|Casting|CastToBP_Hero (Game|Player|GetPlayerPawn 0)))
  (Variables|Default|SetCharacter _asbp_hero)
  (EventDispatchers|AssignUseItem (Variables|Default|GetInventoryWidget) (delegate Custom|UseItem_Event)))

(event EventTick
  (params (DeltaSeconds :type Float%20%28single-precision%29)))