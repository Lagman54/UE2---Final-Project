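; Player hero character for a third-person shooter, handling Enhanced Input movement, sprinting, aiming, shooting, reloading, interaction and death.
; Aiming gates firing, switches rotation mode and shortens the spring arm via a timeline.
; Weapon switching respawns a socket-attached pistol or shotgun (enum Rifle), while montages time shotgun fire and reloads.
; Camera sphere traces call BPI_Interactible, lock and HUD functions suspend control or display, and death ragdolls and notifies BP_GI.
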(event Custom|Update%20Ammo%20HUD)

(event Custom|Start%20Aim
  (bind _charactermovement (Variables|Character|GetCharacterMovement))
  ;[0.15 0.15 0.15 0.5] Aim
  (if (Variables|Default|GetAimingAllowed)
    (Variables|/Script/Engine.CharacterMovementComponent|SetbOrientRotationToMovement _charactermovement false)
    (Variables|/Script/Engine.CharacterMovementComponent|SetbUseControllerDesiredRotation _charactermovement true)
    (CallFunction|Walk)
    (Variables|Default|SetIsAiming true)
    (Widget|SetVisibility (Variables|Default|GetAimWidget) "Visible")
    (bind _newtrack_0 (Timeline|Timeline Play)
      (:Update
        (Variables|/Script/Engine.SpringArmComponent|SetTargetArmLength (Variables|Default|GetSpringArm) (Math|Float|Lerp 2e+02 1e+02 _newtrack_0))))))

(event Custom|Release%20Aim
  (bind _charactermovement (Variables|Character|GetCharacterMovement))
  ;[0.15 0.15 0.15 0.5] Aim
  (if (Variables|Default|GetIsAiming)
    (Variables|/Script/Engine.CharacterMovementComponent|SetbOrientRotationToMovement _charactermovement true)
    (Variables|/Script/Engine.CharacterMovementComponent|SetbUseControllerDesiredRotation _charactermovement false)
    (Variables|Default|SetIsAiming false)
    (Widget|SetVisibility (Variables|Default|GetAimWidget) "Hidden")
    (bind _newtrack_0 (Timeline|Timeline Reverse)
      (:Update
        (Variables|/Script/Engine.SpringArmComponent|SetTargetArmLength (Variables|Default|GetSpringArm) (Math|Float|Lerp 2e+02 1e+02 _newtrack_0))))))

(event Custom|PlayReloadAnim
  (bind _currentweaponbp (Variables|Default|GetCurrentWeaponBP))
  ;[0.15 0.15 0.15 0.5] Reload
  (Variables|/Game/Blueprints/Weapons/BP_BaseWeapon.BP_BaseWeapon_C|SetIsReloading _currentweaponbp true)
  (Animation|Montage|PlayMontage (Variables|Character|GetMesh) "/Game/Animation/Rifle/Reloading_Montage.Reloading_Montage" 1.0 0.0 "None" false
    (:OnCompleted
      (Variables|/Game/Blueprints/Weapons/BP_BaseWeapon.BP_BaseWeapon_C|SetIsReloading _currentweaponbp false)
      (Default|Reload _currentweaponbp))))

(event Custom|ReloadGun
  ;[0.15 0.15 0.15 0.5] Reload
  (bind _result (Default|CanReload (Variables|Default|GetCurrentWeaponBP)))
  (if _result
    (CallFunction|PlayReloadAnim)))

(event Input|EnhancedActionEvents|EnhancedInputActionIA_Switch_Weapon
  (params (ActionValue :type Float%20%28double-precision%29) (ElapsedSeconds :type Float%20%28double-precision%29) (TriggeredSeconds :type Float%20%28double-precision%29) (InputAction :type Input%20Action%20Object%20Reference :default "/Game/Character/Input/IA_Switch_Weapon.IA_Switch_Weapon"))
  (bind _returnvalue (|GetNumEnumEntries))
  ;[0.15 0.15 0.15 0.5] Switch Weapon
  (if (not (or (Variables|/Game/Blueprints/Weapons/BP_BaseWeapon.BP_BaseWeapon_C|GetIsReloading (Variables|Default|GetCurrentWeaponBP)) (Variables|Default|GetIsShooting)))
    (if (Variables|/Game/Character/BP_InventoryComponent.BP_InventoryComponent_C|GetHasShotgun? (Variables|Default|GetBP_InventoryComponent))
      (switch string (Utilities|String|ToString(Integer) (Math|Float|Truncate ActionValue))
        (:-1
          (bind _output_get (Variables|Default|SetCurrentWeaponIndex (Math|Integer|%(Integer) (+ (- (Variables|Default|GetCurrentWeaponIndex) 1) _returnvalue) _returnvalue)))
          (CallFunction|SwitchWeapon _output_get))
        (:1
          (bind _output_get_2 (Variables|Default|SetCurrentWeaponIndex (Math|Integer|%(Integer) (+ (Variables|Default|GetCurrentWeaponIndex) 1) (|GetNumEnumEntries))))
          (CallFunction|SwitchWeapon _output_get_2)))
      (Development|PrintString (Utilities|String|EnumtoString (Variables|Default|GetCurrentWeapon))))))

(event Input|EnhancedActionEvents|EnhancedInputActionIA_Shoot
  (params (ActionValue :type Boolean) (ElapsedSeconds :type Float%20%28double-precision%29) (TriggeredSeconds :type Float%20%28double-precision%29) (InputAction :type Input%20Action%20Object%20Reference :default "/Game/Character/Input/IA_Shoot.IA_Shoot"))
  (bind _currentweaponbp (Variables|Default|GetCurrentWeaponBP))
  ;[0.15 0.15 0.15 0.5] Shooting
  (:Started
    (if (not (Variables|Default|GetIsCharacterLocked))
      (if (Variables|Default|GetIsShooting)
        (Development|PrintString "shooting")
        (else
          (Utilities|IsValid _currentweaponbp
            (:Is%20Valid
              (if (Variables|Default|GetIsAiming)
                (Variables|Default|SetIsShooting true)
                (Default|Shoot _currentweaponbp)
                (switch Utilities|FlowControl|Switch|SwitchonE_WeaponType (Variables|Default|GetCurrentWeapon)
                  (:NewEnumerator0
                    _)
                  (:NewEnumerator1
                    (Animation|Montage|PlayMontage (Variables|Character|GetMesh) "/Game/Animation/Rifle/Rifle_Firing_Montage.Rifle_Firing_Montage" 1.0 0.0 "None" false
                      (:OnCompleted
                        _))))
                (Variables|Default|SetIsShooting false)
                (if (<= (Variables|/Game/Blueprints/Weapons/BP_BaseWeapon.BP_BaseWeapon_C|GetAmmo (Variables|Default|GetCurrentWeaponBP)) 0)
                  (CallFunction|ReloadGun))))))))))

(event Input|EnhancedActionEvents|EnhancedInputActionIA_Reload
  (params (ActionValue :type Boolean) (ElapsedSeconds :type Float%20%28double-precision%29) (TriggeredSeconds :type Float%20%28double-precision%29) (InputAction :type Input%20Action%20Object%20Reference :default "/Game/Character/Input/IA_Reload.IA_Reload"))
  ;[0.15 0.15 0.15 0.5] Reload
  (if (not (Variables|Default|GetIsCharacterLocked))
    (CallFunction|ReloadGun)))

(event Input|EnhancedActionEvents|EnhancedInputActionIA_Interact
  (params (ActionValue :type Boolean) (ElapsedSeconds :type Float%20%28double-precision%29) (TriggeredSeconds :type Float%20%28double-precision%29) (InputAction :type Input%20Action%20Object%20Reference :default "/Game/Character/Input/IA_Interact.IA_Interact"))
  (bind _camera (Variables|Default|GetCamera))
  (bind _springarm (Variables|Default|GetSpringArm))
  (bind _returnvalue (Transformation|GetWorldLocation _camera))
  (bind _returnvalue_2 (Math|Vector|GetForwardVector _camera))
  (bind _targetarmlength (Variables|/Script/Engine.SpringArmComponent|GetTargetArmLength _springarm))
  (bind _returnvalue_3 (* _returnvalue_2 _targetarmlength))
  (bind _returnvalue_4 (+ _returnvalue _returnvalue_3))
  ;[0.15 0.15 0.15 0.5] Interaction
  (:Started
    (if (not (Variables|Default|GetIsCharacterLocked))
      (bind _outhit (Collision|SphereTraceByChannel _returnvalue_4 (+ _returnvalue_4 (* _returnvalue_2 "300.000000,300.000000,300.000000")) 16.0 "TraceTypeQuery1" false 0 "ForDuration"))
      (bind _asbpi_interactible (Utilities|Casting|CastToBPI_Interactible (.HitActor (Collision|BreakHitResult _outhit))))
      (Default|OnInteract _asbpi_interactible))))

(event Input|EnhancedActionEvents|EnhancedInputActionIA_Look
  (params (ActionValue :type Vector%202D%20Structure) (ElapsedSeconds :type Float%20%28double-precision%29) (TriggeredSeconds :type Float%20%28double-precision%29) (InputAction :type Input%20Action%20Object%20Reference :default "/Game/Character/Input/IA_Look.IA_Look"))
  ;[0.15 0.15 0.15 0.5] IA_Look
  (if (not (Variables|Default|GetIsCharacterLocked))
    (Pawn|Input|AddControllerYawInput (.x ActionValue))
    (bind _result (Math|Float|NegateFloat (.y ActionValue))
      (:%20%20
        (Pawn|Input|AddControllerPitchInput _result)))))

(event Input|EnhancedActionEvents|EnhancedInputActionIA_Move
  (params (ActionValue :type Vector%202D%20Structure) (ElapsedSeconds :type Float%20%28double-precision%29) (TriggeredSeconds :type Float%20%28double-precision%29) (InputAction :type Input%20Action%20Object%20Reference :default "/Game/Character/Input/IA_Move.IA_Move"))
  ;[0.15 0.15 0.15 0.5] IA_Move
  (Pawn|Input|AddMovementInput (Math|Vector|GetForwardVector (Math|Rotator|MakeRotator 0.0 0.0 (.yaw (Pawn|GetControlRotation :!class /Script/Engine.Pawn)))) (.x ActionValue) false)
  (Pawn|Input|AddMovementInput (Math|Vector|GetRightVector (Pawn|GetControlRotation :!class /Script/Engine.Pawn)) (.y ActionValue) false))

(event Input|EnhancedActionEvents|EnhancedInputActionIA_Sprint
  (params (ActionValue :type Boolean) (ElapsedSeconds :type Float%20%28double-precision%29) (TriggeredSeconds :type Float%20%28double-precision%29) (InputAction :type Input%20Action%20Object%20Reference :default "/Game/Character/Input/IA_Sprint.IA_Sprint"))
  ;[0.15 0.15 0.15 0.5] Sprint
  (:Started
    (if (not (Variables|Default|GetIsAiming))
      (CallFunction|Sprint)))
  (:Completed
    (CallFunction|Walk)))

(event Input|EnhancedActionEvents|EnhancedInputActionIA_Aim
  (params (ActionValue :type Boolean) (ElapsedSeconds :type Float%20%28double-precision%29) (TriggeredSeconds :type Float%20%28double-precision%29) (InputAction :type Input%20Action%20Object%20Reference :default "/Game/Character/Input/IA_Aim.IA_Aim"))
  (:Started
    (if (not (Variables|Default|GetIsCharacterLocked))
      (CallFunction|StartAim)))
  (:Completed
    (if (not (Variables|Default|GetIsCharacterLocked))
      (CallFunction|ReleaseAim))))

(event EventBeginPlay
  ;[0.15 0.15 0.15 0.5] Event BeginPlay
  (Input|AddMappingContext (PlayerController|LocalPlayerSubsystems|GetEnhancedInputLocalPlayerSubsystem (Game|GetPlayerController 0)) "/Game/Character/Input/IMC_Player.IMC_Player" 0 "(bIgnoreAllPressedKeysUntilRelease=True,bForceImmediately=False,bNotifyUserSettings=False)")
  (bind _returnvalue (UserInterface|CreateWidget "/Game/UI/WBP_Aim.WBP_Aim_C"))
  (bind _output_get (Variables|Default|SetAimWidget _returnvalue))
  (Widget|SetVisibility _output_get "Hidden")
  (bind _returnvalue_2 (UserInterface|CreateWidget "/Game/UI/WBP_HUD.WBP_HUD_C"))
  (bind _output_get_2 (Variables|Default|SetWBP%20HUD _returnvalue_2))
  (UserInterface|Viewport|AddtoViewport (Variables|Default|GetAimWidget) 0)
  (bind _output_get_3 (Variables|Default|SetCurrentWeaponIndex 0))
  (CallFunction|SwitchWeapon _output_get_3)
  (bind _asbp_gi (Utilities|Casting|CastToBP_GI (Game|GetGameInstance)))
  (Variables|Default|SetGame%20Instance _asbp_gi))

(event Game|Damage|EventAnyDamage
  (params (Damage :type Float%20%28single-precision%29) (DamageType :type Damage%20Type%20Object%20Reference) (InstigatedBy :type Controller%20Object%20Reference) (DamageCauser :type Actor%20Object%20Reference))
  (bind _mesh (Variables|Character|GetMesh))
  ;[0.15 0.15 0.15 0.5] Death
  (if (> (Variables|Default|GetHP) 0.0)
    (bind _output_get (Variables|Default|SetHP (- (Variables|Default|GetHP) Damage)))
    (if (<= _output_get 0.0)
      (Physics|SetSimulatePhysics _mesh true)
      (Collision|SetCollisionProfileName _mesh "Ragdoll" true :!class /Script/Engine.PrimitiveComponent)
      (Input|DisableInput 0)
      (Default|Death (Variables|Default|GetGame%20Instance)))))

(event EventTick
  (params (DeltaSeconds :type Float%20%28single-precision%29))
  (bind _returnvalue (Pawn|GetControlRotation :!class /Script/Engine.Pawn))
  (bind _returnvalue_2 (Math|Float|ClampAngle (.pitch _returnvalue) -8e+01 5e+01))
  ;[0.15 0.15 0.15 0.5] Event Tick
  (Pawn|SetControlRotation (Game|GetPlayerController 0) (Math|Rotator|MakeRotator (.roll _returnvalue) _returnvalue_2 (.yaw _returnvalue)))
  (Variables|Default|SetRealPitch _returnvalue_2))

(fn ConstructionScript)

(fn Sprint
  (Variables|/Script/Engine.CharacterMovementComponent|SetMaxWalkSpeed (Variables|Character|GetCharacterMovement) 6e+02)
  (Variables|Default|SetIsSprinting true))

(fn Walk
  (Variables|/Script/Engine.CharacterMovementComponent|SetMaxWalkSpeed (Variables|Character|GetCharacterMovement) 4e+02)
  (Variables|Default|SetIsSprinting false))

(fn SwitchWeapon
  (params (Weapon%20Index :type Integer))
  (switch string (Utilities|String|ToString(Integer) Weapon%20Index)
    (:0
      (Variables|Default|SetCurrentWeapon "NewEnumerator0")
      (Utilities|IsValid (Variables|Default|GetCurrentWeaponBP)
        (:Is%20Valid
          (Actor|DestroyActor (Variables|Default|GetCurrentWeaponBP)))
        (:Is%20Not%20Valid
          _))
      (bind _returnvalue (Game|SpawnActorfromClass "/Game/Blueprints/Weapons/BP_Pistol.BP_Pistol_C" (Transformation|GetActorTransform) "Undefined" "MultiplyWithRoot" 0 0))
      (bind _output_get (Variables|Default|SetCurrentWeaponBP _returnvalue))
      (Transformation|AttachComponentToComponent _output_get (Variables|Character|GetMesh) "Rifle_Idle_Socket" "SnapToTarget" "SnapToTarget" "SnapToTarget" true))
    (:1
      (Variables|Default|SetCurrentWeapon "NewEnumerator1")
      (Utilities|IsValid (Variables|Default|GetCurrentWeaponBP)
        (:Is%20Valid
          (Actor|DestroyActor (Variables|Default|GetCurrentWeaponBP)))
        (:Is%20Not%20Valid
          _))
      (bind _returnvalue_2 (Game|SpawnActorfromClass "/Game/Blueprints/Weapons/BP_Shotgun.BP_Shotgun_C" (Transformation|GetActorTransform) "Undefined" "MultiplyWithRoot" 0 0))
      (bind _output_get_2 (Variables|Default|SetCurrentWeaponBP _returnvalue_2))
      (Transformation|AttachComponentToComponent _output_get_2 (Variables|Character|GetMesh) "Rifle_Idle_Socket" "SnapToTarget" "SnapToTarget" "SnapToTarget" true))))

(fn LockCharacter
  (Variables|Default|SetIsCharacterLocked true)
  (CallFunction|ReleaseAim)
  (Pawn|Components|CharacterMovement|DisableMovement (Variables|Character|GetCharacterMovement)))

(fn UnlockCharacter
  (Variables|Default|SetIsCharacterLocked false)
  (Pawn|Components|CharacterMovement|SetMovementMode (Variables|Character|GetCharacterMovement) "MOVE_Walking" 0))

(fn HideHUD
  (Widget|RemovefromParent (Variables|Default|GetWBP%20HUD)))

(fn ShowHUD
  (UserInterface|Viewport|AddtoViewport (Variables|Default|GetWBP%20HUD) 0))