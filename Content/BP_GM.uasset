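; BP_GM, likely the game mode by its name, holds a random lion statue code and the spare pistol and shotgun ammo counts.
; The construction script rolls a three-digit code as a string, which BeginPlay prints to screen, apparently for debugging.
; UpdateSpareAmmo switches on ammo type and adds the given amount to the matching spare count, with no clamping.
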(event EventBeginPlay
  (Development|PrintString (Variables|Default|GetLionStatueCode) true true "(R=0.000000,G=0.660000,B=1.000000,A=1.000000)" 2e+01))

(event EventTick
  (params (DeltaSeconds :type Float%20%28single-precision%29)))

(fn ConstructionScript
  (Variables|Default|SetLionStatueCode (Utilities|String|ToString(Integer) (Math|Random|RandomIntegerinRange 100 999))))

(fn UpdateSpareAmmo
  (params (Ammo%20Type :type String) (Amount :type Integer))
  (switch string Ammo%20Type
    (:Pistol%20Ammo
      (Variables|Default|SetPistolAmmoSpare (+ (Variables|Default|GetPistolAmmoSpare) Amount)))
    (:Shotgun%20Ammo
      (Variables|Default|SetShotgunAmmoSpare (+ (Variables|Default|GetShotgunAmmoSpare) Amount)))))