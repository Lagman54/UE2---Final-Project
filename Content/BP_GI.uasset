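; Game instance Blueprint that handles level restart and the game's win and loss screens.
; Restart reopens the current level by looking up its name.
; Death and Win each create their own widget (WBP_GameOver or WBP_Win), add it to the viewport and show the first player's mouse cursor.
; Neither end-state function pauses the game or changes the input mode.
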(fn Restart
  (bind _returnvalue (Game|GetCurrentLevelName true))
  (Game|OpenLevel(byName) (Utilities|String|StringToName _returnvalue)))

(fn Death
  (bind _returnvalue (UserInterface|CreateWidget "/Game/UI/WBP_GameOver.WBP_GameOver_C"))
  (UserInterface|Viewport|AddtoViewport _returnvalue 0)
  (Variables|/Script/Engine.PlayerController|SetbShowMouseCursor (Game|GetPlayerController 0) true))

(fn Win
  (bind _returnvalue (UserInterface|CreateWidget "/Game/UI/WBP_Win.WBP_Win_C"))
  (UserInterface|Viewport|AddtoViewport _returnvalue 0)
  (Variables|/Script/Engine.PlayerController|SetbShowMouseCursor (Game|GetPlayerController 0) true))