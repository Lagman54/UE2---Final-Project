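; BP_Item is a world pickup that the hero can add to their inventory by interacting.
; The construction script configures a physics-simulated mesh and collision sphere scale from the Item data.
; Sphere overlap with BP_Hero shows or hides a "[E] Pick Up" prompt widget.
; OnInteract checks that overlap, passes the actor to the hero's inventory component, and sets HasShotgun for shotgun items.
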(event OnComponentBeginOverlap(CollisionSphere)
  (params (OverlappedComponent :type Primitive%20Component%20Object%20Reference) (OtherActor :type Actor%20Object%20Reference) (OtherComp :type Primitive%20Component%20Object%20Reference) (OtherBodyIndex :type Integer) (bFromSweep :type Boolean) (SweepResult :type Hit%20Result%20Structure%20%28by%20ref%29))
  (Utilities|Casting|CastToBP_Hero OtherActor)
  (Widget|SetVisibility (Variables|Default|GetAs%20WBP%20Interact%20Prompt) "Visible"))

(event OnComponentEndOverlap(CollisionSphere)
  (params (OverlappedComponent :type Primitive%20Component%20Object%20Reference) (OtherActor :type Actor%20Object%20Reference) (OtherComp :type Primitive%20Component%20Object%20Reference) (OtherBodyIndex :type Integer))
  (Utilities|Casting|CastToBP_Hero OtherActor)
  (Widget|SetVisibility (Variables|Default|GetAs%20WBP%20Interact%20Prompt) "Hidden"))

(event EventBeginPlay
  (bind _aswbp_interact_prompt (Utilities|Casting|CastToWBP_InteractPrompt (UserInterface|GetUserWidgetObject (Variables|Default|GetInteractPrompt))))
  (bind _output_get (Variables|Default|SetAs%20WBP%20Interact%20Prompt _aswbp_interact_prompt))
  (Variables|/Game/UI/WBP_InteractPrompt.WBP_InteractPrompt_C|SetPromptText _output_get "[E] Pick Up")
  (Widget|SetVisibility _output_get "Hidden"))

(event Collision|EventActorBeginOverlap
  (params (OtherActor :type Actor%20Object%20Reference)))

(event EventTick
  (params (DeltaSeconds :type Float%20%28single-precision%29)))

(event EventOnInteract
  (bind _self self)
  (bind _result (CallFunction|CanInteract))
  (if _result
    (bind _asbp_hero (Utilities|Casting|CastToBP_Hero (Game|GetPlayerCharacter 0)))
    (if (.shotgun? (Variables|Default|GetItem _self))
      (Variables|/Game/Character/BP_InventoryComponent.BP_InventoryComponent_C|SetHasShotgun? (Variables|/Game/Character/BP_Hero.BP_Hero_C|GetBP_InventoryComponent _asbp_hero) true))
    (Default|AddItem (Variables|/Game/Character/BP_Hero.BP_Hero_C|GetBP_InventoryComponent _asbp_hero) _self)))

(fn ConstructionScript
  (bind _item (Variables|Default|GetItem))
  (bind _staticmesh (Variables|Default|GetStaticMesh))
  (bind (_name _stackable _quantity _thumbnail _mesh _meshscale _collisionscale) (Utilities|Struct|BreakS_ItemStructure _item))
  (Components|StaticMesh|SetStaticMesh (Variables|Default|GetStaticMesh) _mesh)
  (Physics|SetSimulatePhysics _staticmesh true)
  (Transformation|SetWorldScale3D _staticmesh (Math|Vector|MakeVector _meshscale _meshscale _meshscale))
  (Transformation|SetWorldScale3D (Variables|Default|GetCollision%20Sphere) (Math|Vector|MakeVector _collisionscale _collisionscale _collisionscale)))

(fn CanInteract
  (return (Collision|IsOverlappingActor (Variables|Default|GetCollision%20Sphere) (Game|GetPlayerCharacter 0) :!class /Script/Engine.PrimitiveComponent)))