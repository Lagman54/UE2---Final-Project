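; Shotgun weapon Blueprint that specializes a parent weapon with spread hitscan fire, its own pitched-down shot sound and a small capacity.
; Each shot trace event fires multiple camera-based line traces within a narrow random cone, applying base damage per hit, with debug drawing left on.
; It loads loaded and spare ammo from BPGM on BeginPlay and writes both back in UpdateGM, while Shoot defers to the parent.
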(event EventBeginPlay
  (bind _bp_gm (Variables|Default|GetBP_GM))
  (|CallParentFunction)
  (Variables|Default|SetCapacity 5)
  (Variables|Default|SetAmmo (Variables|/Game/BP_GM.BP_GM_C|GetShotgunAmmo _bp_gm))
  (Variables|Default|SetSpareAmmo (Variables|/Game/BP_GM.BP_GM_C|GetShotgunAmmoSpare _bp_gm)))

(event Collision|EventActorBeginOverlap
  (params (OtherActor :type Actor%20Object%20Reference))
  (|CallParentFunction OtherActor) ; This node is disabled and will not be called.\nDrag off pins to build functionality.
)

(event EventTick
  (params (DeltaSeconds :type Float%20%28single-precision%29))
  (|CallParentFunction DeltaSeconds) ; This node is disabled and will not be called.\nDrag off pins to build functionality.
)

(event EventShoot
  (|CallParentFunction))

(event EventPlayShotSound
  (Audio|PlaySound2D "/Game/SFX/GunShot_1.GunShot_1" 1.0 0.8 0.0 0 0))

(event EventCreateShotTrace
  (params (Range :type Float%20%28double-precision%29))
  (bind _character (Variables|Default|GetCharacter))
  (bind _camera (Variables|/Game/Character/BP_Hero.BP_Hero_C|GetCamera _character))
  (bind _returnvalue (Transformation|GetWorldLocation _camera))
  (for _index (range 0 8)
    (bind (_outhit _returnvalue_2) (Collision|LineTraceByChannel (+ (* (Math|Vector|GetForwardVector (Transformation|GetWorldRotation _camera)) 150) _returnvalue) (+ _returnvalue (* (Math|Random|RandomUnitVectorinConeinDegrees (Math|Vector|GetForwardVector (Transformation|GetWorldRotation (Variables|/Game/Character/BP_Hero.BP_Hero_C|GetCamera (Variables|Default|GetCharacter)))) 4.0) Range)) "TraceTypeQuery2" false 0 "ForDuration"))
    (if _returnvalue_2
      (Game|Damage|ApplyDamage (.HitActor (Collision|BreakHitResult _outhit)) (Variables|Default|GetWeaponBaseDamage) 0 0))))

(event EventUpdateGM
  (bind _bp_gm (Variables|Default|GetBP_GM))
  (Variables|/Game/BP_GM.BP_GM_C|SetShotgunAmmo _bp_gm (Variables|Default|GetAmmo))
  (Variables|/Game/BP_GM.BP_GM_C|SetShotgunAmmoSpare _bp_gm (Variables|Default|GetSpareAmmo)))

(fn ConstructionScript
  (|CallParentFunction))