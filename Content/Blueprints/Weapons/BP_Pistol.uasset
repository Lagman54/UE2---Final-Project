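; BP_Pistol is a pistol weapon Blueprint built on a parent weapon class that supplies the shooting logic.
; On BeginPlay it sets a ten-round capacity and loads its loaded and spare ammo from the BPGM reference.
; UpdateGM writes both ammo counts back to BPGM, so ammo state is stored outside the weapon.
; Shoot defers to the parent, and PlayShotSound plays the gunshot as a non-spatial 2D sound.
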(event EventBeginPlay
  (bind _bp_gm (Variables|Default|GetBP_GM))
  (|CallParentFunction)
  (Variables|Default|SetCapacity 10)
  (Variables|Default|SetAmmo (Variables|/Game/BP_GM.BP_GM_C|GetPistolAmmo _bp_gm))
  (Variables|Default|SetSpareAmmo (Variables|/Game/BP_GM.BP_GM_C|GetPistolAmmoSpare _bp_gm)))

(event Collision|EventActorBeginOverlap
  (params (OtherActor :type Actor%20Object%20Reference))
  (|CallParentFunction OtherActor) ; This node is disabled and will not be called.\nDrag off pins to build functionality.
)

(event EventTick
  (params (DeltaSeconds :type Float%20%28single-precision%29))
  (|CallParentFunction DeltaSeconds) ; This node is disabled and will not be called.\nDrag off pins to build functionality.
)

(event EventShoot
  (|CallParentFunction))

(event EventPlayShotSound
  (Audio|PlaySound2D "/Game/SFX/GunShot_1.GunShot_1" 1.0 1.0 0.0 0 0))

(event EventUpdateGM
  (bind _bp_gm (Variables|Default|GetBP_GM))
  (Variables|/Game/BP_GM.BP_GM_C|SetPistolAmmo _bp_gm (Variables|Default|GetAmmo))
  (Variables|/Game/BP_GM.BP_GM_C|SetPistolAmmoSpare _bp_gm (Variables|Default|GetSpareAmmo)))

(fn ConstructionScript
  (|CallParentFunction))