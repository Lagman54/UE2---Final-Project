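; Zombie enemy that wanders, chases and attacks the hero, and reacts to damage.
; It patrols slowly to random reachable points around its spawn location until PawnSensing spots BP_Hero, then runs at it with AIMoveTo.
; On arrival an attack montage's notify fires a forward sphere trace to apply damage.
; Damage triggers a stagger or death montage, with CanMove blocking new movement while staggered or dead.
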(event OnSeePawn(PawnSensing)
  (params (Pawn :type Pawn%20Object%20Reference))
  (bind _result (CallFunction|CanMove))
  (if _result
    (bind _asbp_hero (Utilities|Casting|CastToBP_Hero Pawn))
    (CallFunction|ChaseTarget _asbp_hero)))

(event Custom|Chase%20Target
  (params (Target%20Pawn :type Pawn%20Object%20Reference))
  (bind _returnvalue (Transformation|GetActorLocation))
  (bind _result (CallFunction|CanMove))
  (if _result
    (Variables|/Script/Engine.CharacterMovementComponent|SetMaxWalkSpeed (Variables|Character|GetCharacterMovement) 3e+02)
    (AI|AIMoveTo self "0, 0, 0" Target%20Pawn 1.2e+02 false
      (:OnSuccess
        (if (Variables|Default|GetcanAttack)
          (Variables|Default|SetcanAttack false)
          (Animation|Montage|PlayMontage (Variables|Character|GetMesh) "/Game/Blueprints/Zombie/Animation/Zombie_Attack_Montage.Zombie_Attack_Montage"
            (:OnCompleted
              (Variables|Default|SetcanAttack true :!label _label))
            (:OnInterrupted
              (goto _label))
            (:OnNotifyBegin
              (bind (_outhit _returnvalue_2) (Collision|SphereTraceByChannel _returnvalue (+ _returnvalue (* (Math|Vector|GetForwardVector (Transformation|GetActorRotation)) 2e+02)) 2e+01 "TraceTypeQuery2" false 0 "ForDuration"))
              (if _returnvalue_2
                (Game|Damage|ApplyDamage (.HitActor (Collision|BreakHitResult _outhit)) 25.0 0 0)))))))))

(event Custom|Patrol
  (bind _result (CallFunction|CanMove))
  (if _result
    (Variables|/Script/Engine.CharacterMovementComponent|SetMaxWalkSpeed (Variables|Character|GetCharacterMovement) 4e+01)
    (AI|AIMoveTo self (.RandomLocation (AI|Navigation|GetRandomReachablePointinRadius (Variables|Default|GetStartLocation) (Variables|Default|GetPatrol%20Radius) 0 0)) 0 5.0 false
      (:OnSuccess
        (Utilities|FlowControl|Delay 0.0))
      (:OnFail
        _))
    (CallFunction|Patrol)))

(event EventBeginPlay
  (CallFunction|Patrol))

(event Collision|EventActorBeginOverlap
  (params (OtherActor :type Actor%20Object%20Reference)))

(event EventTick
  (params (DeltaSeconds :type Float%20%28single-precision%29)))

(event Game|Damage|EventAnyDamage
  (params (Damage :type Float%20%28single-precision%29) (DamageType :type Damage%20Type%20Object%20Reference) (InstigatedBy :type Controller%20Object%20Reference) (DamageCauser :type Actor%20Object%20Reference))
  (if (Variables|Default|GetIsAlive)
    (bind _output_get (Variables|Default|SetHP (- (Variables|Default|GetHP) Damage)))
    (if (<= _output_get 0.0)
      (Variables|Default|SetIsAlive false)
      (Components|Movement|StopMovementImmediately (Variables|Character|GetCharacterMovement))
      (Animation|Montage|PlayMontage (Variables|Character|GetMesh) "/Game/Blueprints/Zombie/Animation/Zombie_Dying_Montage.Zombie_Dying_Montage"
        (:OnNotifyBegin
          (Collision|SetCollisionEnabled (Variables|Collision|GetCapsuleComponent) "NoCollision")))
      (else
        (Components|Movement|StopMovementImmediately (Variables|Character|GetCharacterMovement))
        (Variables|Default|SetIsStaggered true)
        (Animation|Montage|PlayMontage (Variables|Character|GetMesh) "/Game/Blueprints/Zombie/Animation/Zombie_Reaction_Hit_Montage.Zombie_Reaction_Hit_Montage"
          (:OnCompleted
            (CallFunction|Patrol))
          (:OnNotifyBegin
            (Variables|Default|SetIsStaggered false)))))))

(fn ConstructionScript
  (Variables|Default|SetStartLocation (Transformation|GetActorLocation)))

(fn CanMove
  (if (or (not (Variables|Default|GetIsAlive)) (Variables|Default|GetIsStaggered))
    (return false)
    (else
      (return true))))