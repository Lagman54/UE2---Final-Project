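; Interactable door that swings open and closed on interaction while the player stands inside its trigger box.
; A Timeline lerps the Scene component's yaw from its starting value by Angle, playing forward to open and in reverse to close, with state flags blocking input mid-swing.
; A widget prompt shows for an overlapping BP_Hero, switches between Open and Close text, hides during movement and rechecks overlap shortly afterward.
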(event OnComponentBeginOverlap(Box)
  (params (OverlappedComponent :type Primitive%20Component%20Object%20Reference) (OtherActor :type Actor%20Object%20Reference) (OtherComp :type Primitive%20Component%20Object%20Reference) (OtherBodyIndex :type Integer) (bFromSweep :type Boolean) (SweepResult :type Hit%20Result%20Structure%20%28by%20ref%29))
  (Utilities|Casting|CastToBP_Hero OtherActor)
  (Rendering|SetVisibility (Variables|Default|GetInteractPrompt) true false))

(event OnComponentEndOverlap(Box)
  (params (OverlappedComponent :type Primitive%20Component%20Object%20Reference) (OtherActor :type Actor%20Object%20Reference) (OtherComp :type Primitive%20Component%20Object%20Reference) (OtherBodyIndex :type Integer))
  (Utilities|Casting|CastToBP_Hero OtherActor)
  (Rendering|SetVisibility (Variables|Default|GetInteractPrompt) false false))

(event Custom|Check%20Collision
  (if (Utilities|Array|IsNotEmpty (Collision|GetOverlappingActors (Variables|Default|GetBox) "/Game/Character/BP_Hero.BP_Hero_C" :!class /Script/Engine.PrimitiveComponent))
    (Rendering|SetVisibility (Variables|Default|GetInteractPrompt) true false)))

(event Custom|Close
  (bind _scene (Variables|Default|GetScene))
  (bind _as_wbp_interact_prompt (Variables|Default|GetAs%20WBP%20Interact%20Prompt))
  (bind _initr (Variables|Default|GetInitR))
  (bind _returnvalue (Transformation|GetWorldRotation _scene))
  (if (not (or (Variables|Default|GetIsMoving) (not (Variables|Default|GetIsOpen))))
    (Utilities|IsValid _as_wbp_interact_prompt
      (:Is%20Valid
        (Variables|/Game/UI/WBP_InteractPrompt.WBP_InteractPrompt_C|SetPromptText _as_wbp_interact_prompt "[E] Open")
        (Rendering|SetVisibility (Variables|Default|GetInteractPrompt) false false)
        (Variables|Default|SetIsMoving true)
        (bind _newtrack_1 (Timeline|Timeline Reverse)
          (:Update
            (Transformation|SetWorldRotation _scene (Math|Rotator|MakeRotator (.roll _returnvalue) (.pitch _returnvalue) (Math|Float|Lerp _initr (+ _initr (Variables|Default|GetAngle)) _newtrack_1)) false false))
          (:Finished
            (Variables|Default|SetIsMoving false)
            (Variables|Default|SetIsOpen (not (Variables|Default|GetIsOpen)))
            (Utilities|FlowControl|Delay 0.2)
            (CallFunction|CheckCollision)))))))

(event Custom|Open
  (bind _scene (Variables|Default|GetScene))
  (bind _as_wbp_interact_prompt (Variables|Default|GetAs%20WBP%20Interact%20Prompt))
  (bind _returnvalue (Transformation|GetWorldRotation _scene))
  (if (not (or (Variables|Default|GetIsMoving) (Variables|Default|GetIsOpen)))
    (Utilities|IsValid _as_wbp_interact_prompt
      (:Is%20Valid
        (Variables|/Game/UI/WBP_InteractPrompt.WBP_InteractPrompt_C|SetPromptText _as_wbp_interact_prompt "[E] Close")
        (Rendering|SetVisibility (Variables|Default|GetInteractPrompt) false false)
        (Variables|Default|SetIsMoving true)
        (Variables|Default|SetInitR (.yaw (Transformation|GetWorldRotation (Variables|Default|GetScene))))
        (bind _newtrack_1 (Timeline|Timeline Play)
          (:Update
            (Transformation|SetWorldRotation _scene (Math|Rotator|MakeRotator (.roll _returnvalue) (.pitch _returnvalue) (Math|Float|Lerp (Variables|Default|GetInitR) (+ (Variables|Default|GetInitR) (Variables|Default|GetAngle)) _newtrack_1)) false false))
          (:Finished
            (Variables|Default|SetIsMoving false)
            (Variables|Default|SetIsOpen (not (Variables|Default|GetIsOpen)))
            (Utilities|FlowControl|Delay 0.2)
            (CallFunction|CheckCollision)))))))

(event EventBeginPlay
  (bind _aswbp_interact_prompt (Utilities|Casting|CastToWBP_InteractPrompt (UserInterface|GetUserWidgetObject (Variables|Default|GetInteractPrompt))))
  (bind _output_get (Variables|Default|SetAs%20WBP%20Interact%20Prompt _aswbp_interact_prompt))
  (Variables|/Game/UI/WBP_InteractPrompt.WBP_InteractPrompt_C|SetPromptText _output_get "[E] Open")
  (Rendering|SetVisibility (Variables|Default|GetInteractPrompt) false false))

(event Collision|EventActorBeginOverlap
  (params (OtherActor :type Actor%20Object%20Reference)))

(event EventTick
  (params (DeltaSeconds :type Float%20%28single-precision%29)))

(event EventOnInteract
  (bind _result (CallFunction|CanInteract))
  (if _result
    (if (Variables|Default|GetIsOpen)
      (CallFunction|Close)
      (else
        (CallFunction|Open)))))

(fn ConstructionScript)

(fn CanInteract
  (bind _box (Variables|Default|GetBox))
  (Utilities|IsValid _box
    (:Is%20Valid
      (return (Collision|IsOverlappingActor _box (Game|GetPlayerCharacter 0) :!class /Script/Engine.PrimitiveComponent)))))