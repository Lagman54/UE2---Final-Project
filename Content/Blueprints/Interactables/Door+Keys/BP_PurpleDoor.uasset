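; Purple variant of a key-locked door, built as a child Blueprint that inherits its behavior from a parent class.
; BeginPlay runs the parent logic, then sets KeyID to the purple key identifier.
; The Unlock override and construction script only forward to the parent, and the overlap and tick events are disabled stubs.
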(event EventBeginPlay
  (|CallParentFunction)
  (Variables|Default|SetKeyID "purple key"))

(event Collision|EventActorBeginOverlap
  (params (OtherActor :type Actor%20Object%20Reference))
  (|CallParentFunction OtherActor) ; This node is disabled and will not be called.\nDrag off pins to build functionality.
)

(event EventTick
  (params (DeltaSeconds :type Float%20%28single-precision%29))
  (|CallParentFunction DeltaSeconds) ; This node is disabled and will not be called.\nDrag off pins to build functionality.
)

(fn ConstructionScript
  (|CallParentFunction))

(fn Unlock
  (params (Key%20ID :type String))
  (bind _result (|CallParentFunction Key%20ID))
  (return _result))