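; Interactable hinged door that can be locked with a key, showing an open/close prompt when BP_Hero is in range.
; Interacting while locked switches to the door's view, hides and locks the hero, forces the inventory open and registers the door as CurrentUnlockable.
; Unlock clears the lock and plays a timeline-driven key insert-and-turn animation before restoring the player view.
; Once unlocked, interaction swings the door by playing or reversing a yaw timeline.
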(event OnComponentBeginOverlap(Box)
  (params (OverlappedComponent :type Primitive%20Component%20Object%20Reference) (OtherActor :type Actor%20Object%20Reference) (OtherComp :type Primitive%20Component%20Object%20Reference) (OtherBodyIndex :type Integer) (bFromSweep :type Boolean) (SweepResult :type Hit%20Result%20Structure%20%28by%20ref%29))
  ;[0.15 0.15 0.15 0.5] Interaction range
  (Utilities|Casting|CastToBP_Hero OtherActor)
  (Rendering|SetVisibility (Variables|Default|GetInteractPrompt) true false))

(event OnComponentEndOverlap(Box)
  (params (OverlappedComponent :type Primitive%20Component%20Object%20Reference) (OtherActor :type Actor%20Object%20Reference) (OtherComp :type Primitive%20Component%20Object%20Reference) (OtherBodyIndex :type Integer))
  ;[0.15 0.15 0.15 0.5] Interaction range
  (Utilities|Casting|CastToBP_Hero OtherActor)
  (Rendering|SetVisibility (Variables|Default|GetInteractPrompt) false false))

(event Custom|Check%20Collision
  (if (Utilities|Array|IsNotEmpty (Collision|GetOverlappingActors (Variables|Default|GetBox) "/Game/Character/BP_Hero.BP_Hero_C" :!class /Script/Engine.PrimitiveComponent))
    (Rendering|SetVisibility (Variables|Default|GetInteractPrompt) true false)))

(event Custom|Close
  (bind _scene (Variables|Default|GetScene))
  (bind _initr (Variables|Default|GetInitR))
  (bind _returnvalue (Transformation|GetWorldRotation _scene))
  ;[0.15 0.15 0.15 0.5] Open/Close animation
  (if (not (or (Variables|Default|GetIsMoving) (not (Variables|Default|GetIsOpen))))
    (Variables|/Game/UI/WBP_InteractPrompt.WBP_InteractPrompt_C|SetPromptText (Variables|Default|GetAs%20WBP%20Interact%20Prompt) "[E] Open")
    (Rendering|SetVisibility (Variables|Default|GetInteractPrompt) false false)
    (Variables|Default|SetIsMoving true)
    (bind _newtrack_1 (Timeline|Timeline Reverse)
      (:Update
        (Transformation|SetWorldRotation _scene (Math|Rotator|MakeRotator (.roll _returnvalue) (.pitch _returnvalue) (Math|Float|Lerp _initr (+ _initr (Variables|Default|GetAngle)) _newtrack_1)) false false))
      (:Finished
        (Variables|Default|SetIsMoving false)
        (Variables|Default|SetIsOpen (not (Variables|Default|GetIsOpen)))
        (Rendering|SetVisibility (Variables|Default|GetInteractPrompt) false false)
        (Utilities|FlowControl|Delay 0.2)
        (CallFunction|CheckCollision)))))

(event Custom|Open
  (bind _scene (Variables|Default|GetScene))
  (bind _returnvalue (Transformation|GetWorldRotation _scene))
  ;[0.15 0.15 0.15 0.5] Open/Close animation
  (if (not (or (Variables|Default|GetIsMoving) (Variables|Default|GetIsOpen)))
    (Variables|/Game/UI/WBP_InteractPrompt.WBP_InteractPrompt_C|SetPromptText (Variables|Default|GetAs%20WBP%20Interact%20Prompt) "[E] Close")
    (Rendering|SetVisibility (Variables|Default|GetInteractPrompt) false false)
    (Variables|Default|SetIsMoving true)
    (Variables|Default|SetInitR (.yaw (Transformation|GetWorldRotation (Variables|Default|GetScene))))
    (bind _newtrack_1 (Timeline|Timeline Play)
      (:Update
        (Transformation|SetWorldRotation _scene (Math|Rotator|MakeRotator (.roll _returnvalue) (.pitch _returnvalue) (Math|Float|Lerp (Variables|Default|GetInitR) (+ (Variables|Default|GetInitR) (Variables|Default|GetAngle)) _newtrack_1)) false false))
      (:Finished
        (Variables|Default|SetIsMoving false)
        (Variables|Default|SetIsOpen (not (Variables|Default|GetIsOpen)))
        (Rendering|SetVisibility (Variables|Default|GetInteractPrompt) false false)
        (Utilities|FlowControl|Delay 0.2)
        (CallFunction|CheckCollision)))))

(event Custom|Key%20Unlock%20Animation
  (bind _bp_key (Variables|Default|GetBP_Key))
  (bind _relativelocation (Variables|/Script/Engine.SceneComponent|GetRelativeLocation _bp_key))
  (Variables|Default|SetAnimation? true)
  (bind _asbp_hero (Utilities|Casting|CastToBP_Hero (Game|GetPlayerCharacter 0)))
  (Default|ForceCloseInventory (Variables|/Game/Character/BP_Hero.BP_Hero_C|GetBP_InventoryComponent _asbp_hero))
  (Rendering|SetVisibility (Variables|Default|GetBP_Key) true false)
  (Utilities|FlowControl|Delay 0.4)
  (Utilities|FlowControl|Sequence
    (:then_0
      (Variables|Default|SetRelative%20Location%20X (.y _relativelocation))
      (bind _newtrack_0 (Timeline|Timeline_1 Play)
        (:Update
          (Transformation|SetRelativeLocation (Variables|Default|GetBP_Key) (Math|Vector|MakeVector (.x _relativelocation) (Math|Float|Lerp (Variables|Default|GetRelative%20Location%20X) (- (Variables|Default|GetRelative%20Location%20X) 1e+01) _newtrack_0) (.z _relativelocation)) false false))))
    (:then_1
      (Utilities|FlowControl|Delay 0.5)
      (bind _newtrack_0_2 (Timeline|Timeline_0 Play)
        (:Update
          (Transformation|SetRelativeRotation (Variables|Default|GetBP_Key) (Math|Rotator|MakeRotator (Math|Float|Lerp 0.0 1.8e+02 _newtrack_0_2) 0.0 -9e+01) false false))))
    (:then_2
      (Utilities|FlowControl|Delay 1.1)
      (Timeline|Timeline_0 Reverse))
    (:then_3
      (Utilities|FlowControl|Delay 1.6)
      (Timeline|Timeline_1 Reverse))
    (:then_4
      (Utilities|FlowControl|Delay 2.7)
      (Variables|Default|SetAnimation? false)
      (CallFunction|ExitCamera)
      (Rendering|SetVisibility (Variables|Default|GetBP_Key) false false))))

(event Custom|Exit%20Camera
  (bind _returnvalue (Game|GetPlayerCharacter 0))
  ;[0.15 0.15 0.15 0.5] Exit the door camera
  (if (not (Variables|Default|GetAnimation?))
    (Game|Player|SetViewTargetwithBlend (Game|GetPlayerController 0) (Game|GetPlayerCharacter 0) 0.0 "VTBlend_Linear" 0.0 false)
    (Input|DisableInput (Game|GetPlayerController 0))
    (bind _asbp_hero (Utilities|Casting|CastToBP_Hero _returnvalue))
    (Default|UnlockCharacter _asbp_hero)
    (Rendering|SetVisibility (Variables|/Script/Engine.Character|GetMesh _returnvalue) true true)
    (Rendering|SetVisibility (Variables|Default|GetInteractPrompt) true false)
    (bind _asbp_hero_2 (Utilities|Casting|CastToBP_Hero (Game|GetPlayerCharacter 0)))
    (Variables|/Game/Character/BP_Hero.BP_Hero_C|SetCurrentUnlockable _asbp_hero_2 0)
    (Default|ForceCloseInventory (Variables|/Game/Character/BP_Hero.BP_Hero_C|GetBP_InventoryComponent _asbp_hero_2))
    (Default|ShowHUD _asbp_hero_2)))

(event EventBeginPlay
  (bind _aswbp_interact_prompt (Utilities|Casting|CastToWBP_InteractPrompt (UserInterface|GetUserWidgetObject (Variables|Default|GetInteractPrompt))))
  (bind _output_get (Variables|Default|SetAs%20WBP%20Interact%20Prompt _aswbp_interact_prompt))
  (Variables|/Game/UI/WBP_InteractPrompt.WBP_InteractPrompt_C|SetPromptText _output_get "[E] Open")
  (Rendering|SetVisibility (Variables|Default|GetInteractPrompt) false false)
  (Rendering|SetVisibility (Variables|Default|GetBP_Key) false false)
  (Transformation|SetMobility (Variables|Default|GetScene) "Movable"))

(event EventOnInteract
  (bind _returnvalue (Game|GetPlayerCharacter 0))
  (bind _result (CallFunction|CanInteract))
  (if _result
    ;[0.15 0.15 0.15 0.5] Interact
    (bind _asbp_hero (Utilities|Casting|CastToBP_Hero (Game|GetPlayerCharacter 0)))
    (if (Variables|Default|GetIsLocked)
      (Default|ForceOpenInventory (Variables|/Game/Character/BP_Hero.BP_Hero_C|GetBP_InventoryComponent _asbp_hero))
      (Input|EnableInput (Game|GetPlayerController 0))
      (bind _asbp_hero_2 (Utilities|Casting|CastToBP_Hero _returnvalue))
      (Default|LockCharacter _asbp_hero_2)
      (Rendering|SetVisibility (Variables|/Script/Engine.Character|GetMesh _returnvalue) false true)
      (Rendering|SetVisibility (Variables|Default|GetInteractPrompt) false false)
      (Game|Player|SetViewTargetwithBlend (Game|GetPlayerController 0) self 0.0 "VTBlend_Linear" 0.0 false)
      (bind _asbp_hero_3 (Utilities|Casting|CastToBP_Hero (Game|GetPlayerCharacter 0)))
      (Variables|/Game/Character/BP_Hero.BP_Hero_C|SetCurrentUnlockable _asbp_hero_3 self)
      (Default|HideHUD _asbp_hero_3)
      (elif (Variables|Default|GetIsOpen)
        (CallFunction|Close)
        (else
          (CallFunction|Open))))))

(event Input|KeyboardEvents|Backspace
  (params (Key :type Key%20Structure :default "None"))
  (:Pressed
    (CallFunction|ExitCamera)))

(fn ConstructionScript)

(fn CanInteract
  (return (Collision|IsOverlappingActor (Variables|Default|GetBox) (Game|GetPlayerCharacter 0) :!class /Script/Engine.PrimitiveComponent)))

(fn InventoryRestricted?
  (return (Variables|Default|GetAnimation?)))

(fn Unlock
  (params (Key%20ID :type String))
  (if (Utilities|Enum|Equal(Enum) Key%20ID (Variables|Default|GetKeyID))
    (Variables|Default|SetIsLocked false)
    (CallFunction|KeyUnlockAnimation)
    (return false)
    (else
      (return false))))