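; Locked shotgun display shelf that the player opens with an access card to collect a shotgun and ammo.
; Interacting switches to the shelf's camera, locks and hides the hero, opens the inventory and registers the shelf as the current unlockable.
; Unlock plays timelines that lower the card, exit the camera and shrink the window.
; The child-actor items stay non-interactable until that sequence finishes, which also blocks cancelling and inventory use during card movement.
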(event OnComponentBeginOverlap(Box)
  (params (OverlappedComponent :type Primitive%20Component%20Object%20Reference) (OtherActor :type Actor%20Object%20Reference) (OtherComp :type Primitive%20Component%20Object%20Reference) (OtherBodyIndex :type Integer) (bFromSweep :type Boolean) (SweepResult :type Hit%20Result%20Structure%20%28by%20ref%29))
  ;[0.15 0.15 0.15 0.5] Interaction zone
  (if (Variables|Default|GetIsLocked)
    (Utilities|Casting|CastToBP_Hero OtherActor)
    (Rendering|SetVisibility (Variables|Default|GetInteract%20Prompt) true false)))

(event OnComponentEndOverlap(Box)
  (params (OverlappedComponent :type Primitive%20Component%20Object%20Reference) (OtherActor :type Actor%20Object%20Reference) (OtherComp :type Primitive%20Component%20Object%20Reference) (OtherBodyIndex :type Integer))
  ;[0.15 0.15 0.15 0.5] Interaction zone
  (if (Variables|Default|GetIsLocked)
    (Utilities|Casting|CastToBP_Hero OtherActor)
    (Rendering|SetVisibility (Variables|Default|GetInteract%20Prompt) false false)))

(event Custom|Unlock%20Animation
  (bind _accesscard (Variables|Default|GetAccessCard))
  (bind _window_scene (Variables|Default|GetWindow%20Scene))
  (bind _returnvalue (Transformation|GetWorldScale _window_scene))
  (bind _relativelocation (Variables|/Script/Engine.SceneComponent|GetRelativeLocation _accesscard))
  (Variables|Default|SetAnimation? true)
  (bind _asbp_hero (Utilities|Casting|CastToBP_Hero (Game|GetPlayerCharacter 0)))
  (Default|ForceCloseInventory (Variables|/Game/Character/BP_Hero.BP_Hero_C|GetBP_InventoryComponent _asbp_hero))
  (Rendering|SetVisibility (Variables|Default|GetInteract%20Prompt) false false)
  (Rendering|SetVisibility (Variables|Default|GetAccessCard) true false)
  (Utilities|FlowControl|Delay 0.2)
  (bind _output_get (Variables|Default|SetRelative%20Location%20Z (.z _relativelocation)))
  (bind _newtrack_0 (Timeline|Timeline Play)
    (:Update
      (Transformation|SetRelativeLocation (Variables|Default|GetAccessCard) (Math|Vector|MakeVector (.x _relativelocation) (.y _relativelocation) (Math|Float|Lerp (Variables|Default|GetRelative%20Location%20Z) (+ _output_get -13.0) _newtrack_0)) false false))
    (:Finished
      (Variables|Default|SetIsLocked false)
      (Variables|Default|SetAnimation? false)
      (Components|DestroyComponent (Variables|Default|GetBox))
      (Components|DestroyComponent (Variables|Default|GetInteract%20Prompt))
      (Utilities|FlowControl|Delay 0.8)
      (CallFunction|ExitCamera)
      (Utilities|FlowControl|Delay 0.2)
      (Variables|Default|SetReturn%20Value%20X (.x _returnvalue))
      (bind _newtrack_0_2 (Timeline|Timeline_0 Play)
        (:Update
          (Transformation|SetWorldScale3D (Variables|Default|GetWindow%20Scene) (Math|Vector|MakeVector (Math|Float|Lerp (Variables|Default|GetReturn%20Value%20X) 0.0 _newtrack_0_2) (.y _returnvalue) (.z _returnvalue))))
        (:Finished
          (CallFunction|EnableItems))))))

(event Custom|Enable%20items
  (bind _ammobp (Variables|Default|GetAmmoBP))
  (Rendering|SetVisibility (Variables|/Game/Blueprints/Inventory/BP_Item.BP_Item_C|GetInteractPrompt (Variables|Default|GetShotgunBP)) true false)
  (Collision|SetCollisionEnabled (Variables|/Game/Blueprints/Inventory/BP_Item.BP_Item_C|GetCollision%20Sphere (Variables|Default|GetShotgunBP)) "QueryOnly")
  (Rendering|SetVisibility (Variables|/Game/Blueprints/Inventory/BP_Item.BP_Item_C|GetInteractPrompt _ammobp) true false)
  (Collision|SetCollisionEnabled (Variables|/Game/Blueprints/Inventory/BP_Item.BP_Item_C|GetCollision%20Sphere _ammobp) "QueryOnly"))

(event Custom|Exit%20Camera
  (bind _returnvalue (Game|GetPlayerCharacter 0))
  (bind _interact_prompt (Variables|Default|GetInteract%20Prompt))
  ;[0.15 0.15 0.15 0.5] Exit Camera
  (if (not (Variables|Default|GetAnimation?))
    (Game|Player|SetViewTargetwithBlend (Game|GetPlayerController 0) (Game|GetPlayerCharacter 0) 0.0 "VTBlend_Linear" 0.0 false)
    (Input|DisableInput (Game|GetPlayerController 0))
    (bind _asbp_hero (Utilities|Casting|CastToBP_Hero _returnvalue))
    (Default|UnlockCharacter _asbp_hero)
    (Rendering|SetVisibility (Variables|/Script/Engine.Character|GetMesh _returnvalue) true true)
    (Utilities|IsValid _interact_prompt
      (:Is%20Valid
        (Rendering|SetVisibility _interact_prompt true false))
      (:Is%20Not%20Valid
        _))
    (bind _asbp_hero_2 (Utilities|Casting|CastToBP_Hero (Game|GetPlayerCharacter 0)))
    (Variables|/Game/Character/BP_Hero.BP_Hero_C|SetCurrentUnlockable _asbp_hero_2 0)
    (Default|ForceCloseInventory (Variables|/Game/Character/BP_Hero.BP_Hero_C|GetBP_InventoryComponent _asbp_hero_2))
    (Default|ShowHUD _asbp_hero_2)
    (Widget|RemovefromParent (Variables|Default|GetNewVar_0))))

(event EventBeginPlay
  (bind _aswbp_interact_prompt (Utilities|Casting|CastToWBP_InteractPrompt (UserInterface|GetUserWidgetObject (Variables|Default|GetInteract%20Prompt))))
  (bind _output_get (Variables|Default|SetAs%20WBP%20Interact%20Prompt _aswbp_interact_prompt))
  (Variables|/Game/UI/WBP_InteractPrompt.WBP_InteractPrompt_C|SetPromptText _output_get "[E] Use")
  (Rendering|SetVisibility (Variables|Default|GetInteract%20Prompt) false false)
  (Rendering|SetVisibility (Variables|Default|GetAccessCard) false false)
  (bind _asbp_item (Utilities|Casting|CastToBP_Item (Variables|/Script/Engine.ChildActorComponent|GetChildActor (Variables|Default|GetShotgun))))
  (Variables|Default|SetShotgunBP _asbp_item)
  (Physics|SetSimulatePhysics (Variables|/Game/Blueprints/Inventory/BP_Item.BP_Item_C|GetStaticMesh _asbp_item) false)
  (Rendering|SetVisibility (Variables|/Game/Blueprints/Inventory/BP_Item.BP_Item_C|GetInteractPrompt _asbp_item) false false)
  (Collision|SetCollisionEnabled (Variables|/Game/Blueprints/Inventory/BP_Item.BP_Item_C|GetCollision%20Sphere (Variables|Default|GetShotgunBP)) "NoCollision")
  (bind _asbp_item_2 (Utilities|Casting|CastToBP_Item (Variables|/Script/Engine.ChildActorComponent|GetChildActor (Variables|Default|GetAmmo))))
  (bind _output_get_2 (Variables|Default|SetAmmoBP _asbp_item_2))
  (Physics|SetSimulatePhysics (Variables|/Game/Blueprints/Inventory/BP_Item.BP_Item_C|GetStaticMesh _output_get_2) false)
  (Rendering|SetVisibility (Variables|/Game/Blueprints/Inventory/BP_Item.BP_Item_C|GetInteractPrompt _output_get_2) false false)
  (Collision|SetCollisionEnabled (Variables|/Game/Blueprints/Inventory/BP_Item.BP_Item_C|GetCollision%20Sphere _output_get_2) "NoCollision")
  (bind _returnvalue (UserInterface|CreateWidget "/Game/UI/WBP_CancelHUD.WBP_CancelHUD_C"))
  (Variables|Default|SetNewVar_0 _returnvalue))

(event EventOnInteract
  (bind _returnvalue (Game|GetPlayerCharacter 0))
  (bind _result (CallFunction|CanInteract))
  (if _result
    (UserInterface|Viewport|AddtoViewport (Variables|Default|GetNewVar_0) 0)
    ;[0.15 0.15 0.15 0.5] OnInteract
    (bind _asbp_hero (Utilities|Casting|CastToBP_Hero (Game|GetPlayerCharacter 0)))
    (Default|ForceOpenInventory (Variables|/Game/Character/BP_Hero.BP_Hero_C|GetBP_InventoryComponent _asbp_hero))
    (Input|EnableInput (Game|GetPlayerController 0))
    (bind _asbp_hero_2 (Utilities|Casting|CastToBP_Hero _returnvalue))
    (Default|LockCharacter _asbp_hero_2)
    (Rendering|SetVisibility (Variables|/Script/Engine.Character|GetMesh _returnvalue) false true)
    (Rendering|SetVisibility (Variables|Default|GetInteract%20Prompt) false false)
    (Game|Player|SetViewTargetwithBlend (Game|GetPlayerController 0) self 0.0 "VTBlend_Linear" 0.0 false)
    (bind _asbp_hero_3 (Utilities|Casting|CastToBP_Hero (Game|GetPlayerCharacter 0)))
    (Variables|/Game/Character/BP_Hero.BP_Hero_C|SetCurrentUnlockable _asbp_hero_3 self)
    (Default|HideHUD _asbp_hero_3)))

(event Input|KeyboardEvents|Backspace
  (params (Key :type Key%20Structure :default "None"))
  (:Pressed
    (CallFunction|ExitCamera)))

(fn ConstructionScript)

(fn CanInteract
  (if (Variables|Default|GetIsLocked)
    (return (Collision|IsOverlappingActor (Variables|Default|GetBox) (Game|GetPlayerCharacter 0) :!class /Script/Engine.PrimitiveComponent))
    (else
      (return false))))

(fn InventoryRestricted?
  (return (Variables|Default|GetAnimation?)))

(fn Unlock
  (params (Key%20ID :type String))
  (if (Utilities|Enum|Equal(Enum) Key%20ID (Variables|Default|GetKey%20ID))
    (Variables|Default|SetIsLocked false)
    (CallFunction|UnlockAnimation)
    (return false)
    (else
      (return false))))