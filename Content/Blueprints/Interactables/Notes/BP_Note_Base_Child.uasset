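; A note interactable, derived from the base note Blueprint, that reveals the code for the lion medallion.
; On BeginPlay it runs the parent logic, then reads LionStatueCode from BP_GM and appends it as a formatted text entry to Pages.
; The code comes from the game mode at runtime, so the note text is not hardcoded.
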(event EventBeginPlay
  (|CallParentFunction)
  (bind _asbp_gm (Utilities|Casting|CastToBP_GM (Game|GetGameMode)))
  (Utilities|Array|Add (Variables|Default|GetPages) (Utilities|Text|FormatText "Code for lion medalion - {code}" (Variables|/Game/BP_GM.BP_GM_C|GetLionStatueCode _asbp_gm))))

(event Collision|EventActorBeginOverlap
  (params (OtherActor :type Actor%20Object%20Reference))
  (|CallParentFunction OtherActor) ; This node is disabled and will not be called.\nDrag off pins to build functionality.
)

(event EventTick
  (params (DeltaSeconds :type Float%20%28single-precision%29))
  (|CallParentFunction DeltaSeconds) ; This node is disabled and will not be called.\nDrag off pins to build functionality.
)

(fn ConstructionScript
  (|CallParentFunction))