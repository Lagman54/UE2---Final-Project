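; BP_Note_Base is a base actor for readable notes that open a full reader UI when interacted with.
; OnInteract creates a WBP_NoteReader widget, passes it the note's Pages, refreshes it, then pauses the game and switches to UI-only input with a visible cursor.
; CanInteract always returns false, and nothing in this Blueprint closes the reader or unpauses the game.
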(event EventBeginPlay)

(event Collision|EventActorBeginOverlap
  (params (OtherActor :type Actor%20Object%20Reference)))

(event EventTick
  (params (DeltaSeconds :type Float%20%28single-precision%29)))

(event EventOnInteract
  (bind _returnvalue (Game|GetPlayerController 0))
  (bind _returnvalue_2 (UserInterface|CreateWidget "/Game/UI/WBP_NoteReader.WBP_NoteReader_C"))
  (bind _output_get (Variables|Default|SetNote%20WBP _returnvalue_2))
  (Variables|/Game/UI/WBP_NoteReader.WBP_NoteReader_C|SetPages _output_get (Variables|Default|GetPages))
  (UserInterface|Viewport|AddtoViewport (Variables|Default|GetNote%20WBP) 0)
  (Default|RefreshPage (Variables|Default|GetNote%20WBP))
  (Game|SetGamePaused true)
  (Input|SetInputModeUIOnly _returnvalue (Variables|Default|GetNote%20WBP) "DoNotLock" false)
  (Variables|/Script/Engine.PlayerController|SetbShowMouseCursor _returnvalue true))

(fn ConstructionScript)

(fn CanInteract
  (return false))