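; Final statue puzzle interactable that takes the Lion, Mermaid and Unicorn medallions and opens a passage.
; Interacting switches the view to the statue, hides and locks the hero, opens the inventory and registers the statue as CurrentUnlockable.
; Unlock places a matching medallion, removing it from the inventory.
; With all three inserted, chained timelines lower the stand, then the passage scene, blocking camera exit until finished and permanently disabling interaction.
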(event OnComponentBeginOverlap(Box)
  (params (OverlappedComponent :type Primitive%20Component%20Object%20Reference) (OtherActor :type Actor%20Object%20Reference) (OtherComp :type Primitive%20Component%20Object%20Reference) (OtherBodyIndex :type Integer) (bFromSweep :type Boolean) (SweepResult :type Hit%20Result%20Structure%20%28by%20ref%29))
  (Utilities|Casting|CastToBP_Hero OtherActor)
  (Widget|SetVisibility (Variables|Default|GetAs%20WBP%20Interact%20Prompt) "Visible"))

(event OnComponentEndOverlap(Box)
  (params (OverlappedComponent :type Primitive%20Component%20Object%20Reference) (OtherActor :type Actor%20Object%20Reference) (OtherComp :type Primitive%20Component%20Object%20Reference) (OtherBodyIndex :type Integer))
  (Utilities|Casting|CastToBP_Hero OtherActor)
  (Widget|SetVisibility (Variables|Default|GetAs%20WBP%20Interact%20Prompt) "Collapsed"))

(event Custom|Insert%20Lion
  (Rendering|SetVisibility (Variables|Default|GetLion%20Medalion%20Mesh) true false)
  (bind _asbp_hero (Utilities|Casting|CastToBP_Hero (Game|GetPlayerCharacter 0)))
  (Default|DeleteItembyName (Variables|/Game/Character/BP_Hero.BP_Hero_C|GetBP_InventoryComponent _asbp_hero) "Lion Medalion")
  (Variables|Default|SetLion? true)
  (CallFunction|CheckMedalions))

(event Custom|Insert%20Mermaid
  (Rendering|SetVisibility (Variables|Default|GetMermaid%20Medalion%20Mesh) true false)
  (bind _asbp_hero (Utilities|Casting|CastToBP_Hero (Game|GetPlayerCharacter 0)))
  (Default|DeleteItembyName (Variables|/Game/Character/BP_Hero.BP_Hero_C|GetBP_InventoryComponent _asbp_hero) "Mermaid Medalion")
  (Variables|Default|SetMermaid? true)
  (CallFunction|CheckMedalions))

(event Custom|Insert%20Unicorn
  (Rendering|SetVisibility (Variables|Default|GetUnicorn%20Medalion%20Mesh) true false)
  (bind _asbp_hero (Utilities|Casting|CastToBP_Hero (Game|GetPlayerCharacter 0)))
  (Default|DeleteItembyName (Variables|/Game/Character/BP_Hero.BP_Hero_C|GetBP_InventoryComponent _asbp_hero) "Unicorn Medalion")
  (Variables|Default|SetUnicorn? true)
  (CallFunction|CheckMedalions))

(event Custom|Exit%20Camera
  (bind _returnvalue (Game|GetPlayerCharacter 0))
  (bind _interact_prompt (Variables|Default|GetInteract%20Prompt))
  (if (not (Variables|Default|GetAnimation?))
    (Game|Player|SetViewTargetwithBlend (Game|GetPlayerController 0) (Game|GetPlayerCharacter 0) 0.0 "VTBlend_Linear" 0.0 false)
    (Input|DisableInput (Game|GetPlayerController 0))
    (bind _asbp_hero (Utilities|Casting|CastToBP_Hero _returnvalue))
    (Default|UnlockCharacter _asbp_hero)
    (Rendering|SetVisibility (Variables|/Script/Engine.Character|GetMesh _returnvalue) true true)
    (Utilities|IsValid _interact_prompt
      (:Is%20Valid
        (Rendering|SetVisibility _interact_prompt true false))
      (:Is%20Not%20Valid
        _))
    (bind _asbp_hero_2 (Utilities|Casting|CastToBP_Hero (Game|GetPlayerCharacter 0)))
    (Variables|/Game/Character/BP_Hero.BP_Hero_C|SetCurrentUnlockable _asbp_hero_2 0)
    (Default|ForceCloseInventory (Variables|/Game/Character/BP_Hero.BP_Hero_C|GetBP_InventoryComponent _asbp_hero_2))
    (Default|ShowHUD _asbp_hero_2)))

(event Custom|Check%20Medalions
  (if (Math|Boolean|ANDBoolean (Variables|Default|GetLion?) (Variables|Default|GetMermaid?) (Variables|Default|GetUnicorn?))
    (CallFunction|OpenStatue)))

(event Custom|Open%20Statue
  (Variables|Default|SetAnimation? true)
  (Variables|Default|SetIsLocked false)
  (bind _asbp_hero (Utilities|Casting|CastToBP_Hero (Game|GetPlayerCharacter 0)))
  (Default|ForceCloseInventory (Variables|/Game/Character/BP_Hero.BP_Hero_C|GetBP_InventoryComponent _asbp_hero))
  (Components|Activation|SetActive (Variables|Default|GetCamera) false false)
  (Development|PrintString "Opening statue...")
  (Utilities|FlowControl|Delay 0.3)
  (Variables|Default|SetStand%20Location (Transformation|GetWorldLocation (Variables|Default|GetMedialionStand)))
  (bind _newtrack_0 (Timeline|Timeline_0 Play)
    (:Update
      (Transformation|SetWorldLocation (Variables|Default|GetMedialionStand) (Math|Vector|MakeVector (.X (Math|Vector|BreakVector (Variables|Default|GetStand%20Location))) (.Y (Math|Vector|BreakVector (Variables|Default|GetStand%20Location))) (Math|Float|Lerp (.Z (Math|Vector|BreakVector (Variables|Default|GetStand%20Location))) (- (.Z (Math|Vector|BreakVector (Variables|Default|GetStand%20Location))) 6e+01) _newtrack_0)) false false))
    (:Finished
      (Utilities|FlowControl|Delay 0.2)
      (Variables|Default|SetPassage%20Location (Transformation|GetWorldLocation (Variables|Default|GetScene)))
      (bind _newtrack_1 (Timeline|Timeline Play)
        (:Update
          (Transformation|SetWorldLocation (Variables|Default|GetScene) (Math|Vector|MakeVector (.X (Math|Vector|BreakVector (Variables|Default|GetPassage%20Location))) (.Y (Math|Vector|BreakVector (Variables|Default|GetPassage%20Location))) (Math|Float|Lerp (.Z (Math|Vector|BreakVector (Variables|Default|GetPassage%20Location))) (- (.Z (Math|Vector|BreakVector (Variables|Default|GetPassage%20Location))) 2.1e+02) _newtrack_1)) false false))
        (:Finished
          (Variables|Default|SetAnimation? false)
          (Components|DestroyComponent (Variables|Default|GetInteract%20Prompt))
          (CallFunction|ExitCamera))))))

(event EventBeginPlay
  (bind _aswbp_interact_prompt (Utilities|Casting|CastToWBP_InteractPrompt (UserInterface|GetUserWidgetObject (Variables|Default|GetInteract%20Prompt))))
  (bind _output_get (Variables|Default|SetAs%20WBP%20Interact%20Prompt _aswbp_interact_prompt))
  (Variables|/Game/UI/WBP_InteractPrompt.WBP_InteractPrompt_C|SetPromptText _output_get "[E] Inspect")
  (Widget|SetVisibility (Variables|Default|GetAs%20WBP%20Interact%20Prompt) "Hidden")
  (Rendering|SetVisibility (Variables|Default|GetMermaid%20Medalion%20Mesh) false false))

(event EventOnInteract
  (bind _returnvalue (Game|GetPlayerCharacter 0))
  (bind _result (CallFunction|CanInteract))
  (if _result
    (bind _asbp_hero (Utilities|Casting|CastToBP_Hero (Game|GetPlayerCharacter 0)))
    (Default|ForceOpenInventory (Variables|/Game/Character/BP_Hero.BP_Hero_C|GetBP_InventoryComponent _asbp_hero))
    (Input|EnableInput (Game|GetPlayerController 0))
    (bind _asbp_hero_2 (Utilities|Casting|CastToBP_Hero _returnvalue))
    (Default|LockCharacter _asbp_hero_2)
    (Rendering|SetVisibility (Variables|/Script/Engine.Character|GetMesh _returnvalue) false true)
    (Rendering|SetVisibility (Variables|Default|GetInteract%20Prompt) false false)
    (Game|Player|SetViewTargetwithBlend (Game|GetPlayerController 0) self 0.0 "VTBlend_Linear" 0.0 false)
    (bind _asbp_hero_3 (Utilities|Casting|CastToBP_Hero (Game|GetPlayerCharacter 0)))
    (Variables|/Game/Character/BP_Hero.BP_Hero_C|SetCurrentUnlockable _asbp_hero_3 self)
    (Default|HideHUD _asbp_hero_3)))

(event Input|KeyboardEvents|Backspace
  (params (Key :type Key%20Structure :default "None"))
  (:Pressed
    (CallFunction|ExitCamera)))

(fn ConstructionScript)

(fn PutMedalion
  (params (Medalion%20ID :type String))
  (switch string Medalion%20ID
    (:Default
      (Development|PrintString "Cant be used here"))
    (:Lion%20Medalion
      (if (Variables|Default|GetLion?)
        (return false)
        (else
          (CallFunction|InsertLion)
          (return (Variables|Default|GetLion?)))))
    (:Mermaid%20Medalion
      (if (Variables|Default|GetMermaid?)
        (return false)
        (else
          (CallFunction|InsertMermaid)
          (return (Variables|Default|GetMermaid?)))))
    (:Unicorn%20Medalion
      (if (Variables|Default|GetUnicorn?)
        (return false)
        (else
          (CallFunction|InsertUnicorn)
          (return (Variables|Default|GetUnicorn?)))))))

(fn CanInteract
  (if (Variables|Default|GetIsLocked)
    (return (Collision|IsOverlappingActor (Variables|Default|GetBox) (Game|GetPlayerCharacter 0) :!class /Script/Engine.PrimitiveComponent))
    (else
      (return false))))

(fn InventoryRestricted?
  (return (Variables|Default|GetAnimation?)))

(fn Unlock
  (params (Key%20ID :type String))
  (bind _result (CallFunction|PutMedalion Key%20ID))
  (return _result))