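; Lion statue puzzle with a three-digit combination lock that rewards the player with the Lion Medalion.
; Interacting switches to the statue's view, locks and hides the hero, and lets keys cycle highlighted digit planes and increment values.
; Enter checks the code against BP_GM, flashing planes on failure or sliding the medallion out by Timeline on success.
; An Animation flag blocks exit and restricts inventory until E collects the medallion.
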(event OnComponentBeginOverlap(Box)
  (params (OverlappedComponent :type Primitive%20Component%20Object%20Reference) (OtherActor :type Actor%20Object%20Reference) (OtherComp :type Primitive%20Component%20Object%20Reference) (OtherBodyIndex :type Integer) (bFromSweep :type Boolean) (SweepResult :type Hit%20Result%20Structure%20%28by%20ref%29))
  (if (Variables|Default|GetIsLocked)
    (Utilities|Casting|CastToBP_Hero OtherActor)
    (Rendering|SetVisibility (Variables|Default|GetInteract%20Prompt) true false)))

(event OnComponentEndOverlap(Box)
  (params (OverlappedComponent :type Primitive%20Component%20Object%20Reference) (OtherActor :type Actor%20Object%20Reference) (OtherComp :type Primitive%20Component%20Object%20Reference) (OtherBodyIndex :type Integer))
  (if (Variables|Default|GetIsLocked)
    (Utilities|Casting|CastToBP_Hero OtherActor)
    (Rendering|SetVisibility (Variables|Default|GetInteract%20Prompt) false false)))

(event Custom|Select%20Plane
  (params (Plane%20ID :type Integer))
  (switch int Plane%20ID
    (:0
      (Rendering|Material|SetMaterial (Variables|Default|GetPlane0) 0 "/Game/StarterContent/Materials/M_Metal_Chrome.M_Metal_Chrome"))
    (:1
      (Rendering|Material|SetMaterial (Variables|Default|GetPlane1) 0 "/Game/StarterContent/Materials/M_Metal_Chrome.M_Metal_Chrome"))
    (:2
      (Rendering|Material|SetMaterial (Variables|Default|GetPlane2) 0 "/Game/StarterContent/Materials/M_Metal_Chrome.M_Metal_Chrome"))))

(event Custom|Reset%20Planes
  (Rendering|Material|SetMaterial (Variables|Default|GetPlane0) 0 "/Game/StarterContent/Materials/M_Metal_Gold.M_Metal_Gold")
  (Rendering|Material|SetMaterial (Variables|Default|GetPlane1) 0 "/Game/StarterContent/Materials/M_Metal_Gold.M_Metal_Gold")
  (Rendering|Material|SetMaterial (Variables|Default|GetPlane2) 0 "/Game/StarterContent/Materials/M_Metal_Gold.M_Metal_Gold")
  (Variables|Default|SetCurrentPlane 0))

(event Custom|Deselect%20Plane
  (params (Plane%20ID :type Integer))
  (switch int Plane%20ID
    (:0
      (Rendering|Material|SetMaterial (Variables|Default|GetPlane0) 0 "/Game/StarterContent/Materials/M_Metal_Gold.M_Metal_Gold"))
    (:1
      (Rendering|Material|SetMaterial (Variables|Default|GetPlane1) 0 "/Game/StarterContent/Materials/M_Metal_Gold.M_Metal_Gold"))
    (:2
      (Rendering|Material|SetMaterial (Variables|Default|GetPlane2) 0 "/Game/StarterContent/Materials/M_Metal_Gold.M_Metal_Gold"))))

(event Custom|Exit%20Camera
  (bind _returnvalue (Game|GetPlayerCharacter 0))
  (bind _interact_prompt (Variables|Default|GetInteract%20Prompt))
  ;[0.15 0.15 0.15 0.5] Exit Camera
  (if (not (Variables|Default|GetAnimation?))
    (Game|Player|SetViewTargetwithBlend (Game|GetPlayerController 0) (Game|GetPlayerCharacter 0) 0.0 "VTBlend_Linear" 0.0 false)
    (Input|DisableInput (Game|GetPlayerController 0))
    (bind _asbp_hero (Utilities|Casting|CastToBP_Hero _returnvalue))
    (Default|UnlockCharacter _asbp_hero)
    (Rendering|SetVisibility (Variables|/Script/Engine.Character|GetMesh _returnvalue) true true)
    (Utilities|IsValid _interact_prompt
      (:Is%20Valid
        (Rendering|SetVisibility _interact_prompt true false))
      (:Is%20Not%20Valid
        _))
    (bind _asbp_hero_2 (Utilities|Casting|CastToBP_Hero (Game|GetPlayerCharacter 0)))
    (Variables|/Game/Character/BP_Hero.BP_Hero_C|SetCurrentUnlockable _asbp_hero_2 0)
    (Default|ForceCloseInventory (Variables|/Game/Character/BP_Hero.BP_Hero_C|GetBP_InventoryComponent _asbp_hero_2))
    (Default|ShowHUD _asbp_hero_2)
    (Widget|RemovefromParent (Variables|Default|GetWBP%20statue%20HUD))
    (CallFunction|ResetPlanes)))

(event EventBeginPlay
  (bind _aswbp_interact_prompt (Utilities|Casting|CastToWBP_InteractPrompt (UserInterface|GetUserWidgetObject (Variables|Default|GetInteract%20Prompt))))
  (bind _output_get (Variables|Default|SetAs%20WBP%20Interact%20Prompt _aswbp_interact_prompt))
  (Variables|/Game/UI/WBP_InteractPrompt.WBP_InteractPrompt_C|SetPromptText _output_get "[E] Inspect")
  (Rendering|SetVisibility (Variables|Default|GetInteract%20Prompt) false false)
  (bind _aswbp_interact_prompt_2 (Utilities|Casting|CastToWBP_InteractPrompt (UserInterface|GetUserWidgetObject (Variables|Default|GetMedalion%20Prompt))))
  (Variables|/Game/UI/WBP_InteractPrompt.WBP_InteractPrompt_C|SetPromptText _aswbp_interact_prompt_2 "[E] Pick Up")
  (Rendering|SetVisibility (Variables|Default|GetMedalion%20Prompt) false false))

(event Collision|EventActorBeginOverlap
  (params (OtherActor :type Actor%20Object%20Reference)))

(event EventTick
  (params (DeltaSeconds :type Float%20%28single-precision%29)))

(event EventOnInteract
  (bind _returnvalue (Game|GetPlayerCharacter 0))
  (bind _result (CallFunction|CanInteract))
  (if _result
    (Input|EnableInput (Game|GetPlayerController 0))
    (bind _asbp_hero (Utilities|Casting|CastToBP_Hero _returnvalue))
    (Default|LockCharacter _asbp_hero)
    (Rendering|SetVisibility (Variables|/Script/Engine.Character|GetMesh _returnvalue) false true)
    (Rendering|SetVisibility (Variables|Default|GetInteract%20Prompt) false false)
    (Game|Player|SetViewTargetwithBlend (Game|GetPlayerController 0) self 0.0 "VTBlend_Linear" 0.0 false)
    (bind _asbp_hero_2 (Utilities|Casting|CastToBP_Hero (Game|GetPlayerCharacter 0)))
    (Variables|/Game/Character/BP_Hero.BP_Hero_C|SetCurrentUnlockable _asbp_hero_2 self)
    (Default|HideHUD _asbp_hero_2)
    (bind _returnvalue_2 (UserInterface|CreateWidget "/Game/Blueprints/Interactables/LionStatue/WBP_StatueWidget.WBP_StatueWidget_C"))
    (UserInterface|Viewport|AddtoViewport _returnvalue_2 0)
    (Variables|Default|SetWBP%20statue%20HUD _returnvalue_2)
    (CallFunction|SelectPlane)))

(event Input|KeyboardEvents|J
  (params (Key :type Key%20Structure :default "None"))
  (:Pressed
    (CallFunction|DeselectPlane (Variables|Default|GetCurrentPlane))
    (bind _result (Math|Integer|DecrementInt (Variables|Default|GetCurrentPlane))
      (:%20%20
        (if (< _result 0)
          (bind _output_get (Variables|Default|SetCurrentPlane 2))
          (CallFunction|SelectPlane _output_get)
          (else
            (CallFunction|SelectPlane (Variables|Default|GetCurrentPlane))))))))

(event Input|KeyboardEvents|Backspace
  (params (Key :type Key%20Structure :default "None"))
  (:Pressed
    (CallFunction|ExitCamera)))

(event Input|KeyboardEvents|K
  (params (Key :type Key%20Structure :default "None"))
  (:Pressed
    (CallFunction|DeselectPlane (Variables|Default|GetCurrentPlane))
    (bind _result (Math|Integer|IncrementInt (Variables|Default|GetCurrentPlane))
      (:%20%20
        (if (>= _result 3)
          (bind _output_get (Variables|Default|SetCurrentPlane 0))
          (CallFunction|SelectPlane _output_get)
          (else
            (CallFunction|SelectPlane (Variables|Default|GetCurrentPlane))))))))

(event Input|KeyboardEvents|Enter
  (params (Key :type Key%20Structure :default "None"))
  (bind _bitcoin1 (Variables|Default|Getbitcoin1))
  (:Pressed
    (bind _asbp_gm (Utilities|Casting|CastToBP_GM (Game|GetGameMode)))
    (if (and (Utilities|Enum|Equal(Enum) (Variables|/Game/BP_GM.BP_GM_C|GetLionStatueCode _asbp_gm) (Utilities|String|Append (Utilities|String|ToString(Integer) (Variables|Default|GetCode0_Value)) (Utilities|String|ToString(Integer) (Variables|Default|GetCode1_Value)) (Utilities|String|ToString(Integer) (Variables|Default|GetCode2_Value)))) (Variables|Default|GetIsLocked))
      (Variables|Default|SetIsLocked false)
      (Input|DisableInput 0)
      (bind _output_get (Variables|Default|SetInitLocation (Transformation|GetWorldLocation _bitcoin1)))
      (Variables|Default|SetEndLocation (+ _output_get (* (Math|Vector|GetRightVector _bitcoin1) 20)))
      (Widget|RemovefromParent (Variables|Default|GetWBP%20statue%20HUD))
      (Components|Activation|SetActive (Variables|Default|GetCamera) false false)
      (Variables|Default|SetAnimation? true)
      (bind _asbp_hero (Utilities|Casting|CastToBP_Hero (Game|GetPlayerCharacter 0)))
      (Default|ForceCloseInventory (Variables|/Game/Character/BP_Hero.BP_Hero_C|GetBP_InventoryComponent _asbp_hero))
      (bind _newtrack_0 (Timeline|Timeline Play)
        (:Update
          (Transformation|SetWorldLocation (Variables|Default|Getbitcoin1) (Math|Vector|Lerp(Vector) (Variables|Default|GetInitLocation) (Variables|Default|GetEndLocation) _newtrack_0) false false))
        (:Finished
          (Components|DestroyComponent (Variables|Default|GetInteract%20Prompt))
          (Utilities|FlowControl|Delay 1.2)
          (Rendering|SetVisibility (Variables|Default|GetMedalion%20Prompt) true false)
          (Input|EnableInput (Game|GetPlayerController 0))))
      (else
        (Development|PrintString "wrong code")
        (Rendering|Material|SetMaterial (Variables|Default|GetPlane0) 0 "/Engine/VREditor/BasicMeshes/MI_Cube_03.MI_Cube_03")
        (Rendering|Material|SetMaterial (Variables|Default|GetPlane1) 0 "/Engine/VREditor/BasicMeshes/MI_Cube_03.MI_Cube_03")
        (Rendering|Material|SetMaterial (Variables|Default|GetPlane2) 0 "/Engine/VREditor/BasicMeshes/MI_Cube_03.MI_Cube_03")
        (Utilities|FlowControl|Delay 1.0)
        (CallFunction|ResetPlanes)
        (CallFunction|SelectPlane)))))

(event Input|KeyboardEvents|L
  (params (Key :type Key%20Structure :default "None"))
  (:Pressed
    (switch int (Variables|Default|GetCurrentPlane)
      (:0
        (bind _result (Math|Integer|IncrementInt (Variables|Default|GetCode0_Value))
          (:%20%20
            (bind _output_get (Variables|Default|SetCode0_Value (Math|Integer|%(Integer) _result 10)))
            (Rendering|Components|TextRender|SetText (Variables|Default|GetCode0) (Utilities|Text|ToText(Integer) _output_get)))))
      (:1
        (bind _result_2 (Math|Integer|IncrementInt (Variables|Default|GetCode1_Value))
          (:%20%20
            (bind _output_get_2 (Variables|Default|SetCode1_Value (Math|Integer|%(Integer) _result_2 10)))
            (Rendering|Components|TextRender|SetText (Variables|Default|GetCode1) (Utilities|Text|ToText(Integer) _output_get_2)))))
      (:2
        (bind _result_3 (Math|Integer|IncrementInt (Variables|Default|GetCode2_Value))
          (:%20%20
            (bind _output_get_3 (Variables|Default|SetCode2_Value (Math|Integer|%(Integer) _result_3 10)))
            (Rendering|Components|TextRender|SetText (Variables|Default|GetCode2) (Utilities|Text|ToText(Integer) _output_get_3))))))))

(event Input|KeyboardEvents|E
  (params (Key :type Key%20Structure :default "None"))
  (:Pressed
    (Development|PrintString "Hello")
    (if (and (not (Variables|Default|GetIsLocked)) (Rendering|IsVisible (Variables|Default|GetMedalion%20Prompt)))
      (bind _asbp_hero (Utilities|Casting|CastToBP_Hero (Game|GetPlayerCharacter 0)))
      (Default|AddItemS (Variables|/Game/Character/BP_Hero.BP_Hero_C|GetBP_InventoryComponent _asbp_hero) (Utilities|Struct|MakeS_ItemStructure "Lion Medalion" false 1 "/Game/Icons/lion_medalion.lion_medalion" "/Game/Fab/BitCoin/bitcoin/StaticMeshes/bitcoin.bitcoin" 1.0 1.0 false false true true))
      (Components|DestroyComponent (Variables|Default|Getbitcoin1))
      (Components|DestroyComponent (Variables|Default|GetMedalion%20Prompt))
      (Utilities|FlowControl|Delay 1.0)
      (Variables|Default|SetAnimation? false)
      (CallFunction|ExitCamera))))

(fn ConstructionScript)

(fn CanInteract
  (if (Variables|Default|GetIsLocked)
    (return (Collision|IsOverlappingActor (Variables|Default|GetBox) (Game|GetPlayerCharacter 0) :!class /Script/Engine.PrimitiveComponent))
    (else
      (return false))))

(fn InventoryRestricted?
  (return (Variables|Default|GetAnimation?)))

(fn Unlock
  (params (Key%20ID :type String))
  (return false))