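; BP_Locker is an interactable locker that holds a child BP_Item and displays its LockerCode on a label set at construction.
; The item's interact prompt is hidden at BeginPlay.
; Open, while locked, swings WindowScene in yaw on a Timeline, then clears IsLocked and reveals the prompt.
; Unlock and InventoryRestricted both simply return false, so no key or code check happens here.
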(event Custom|Open
  (if (Variables|Default|GetIsLocked)
    (Variables|Default|SetWindow%20Rotation (Transformation|GetWorldRotation (Variables|Default|GetWindow%20Scene)))
    (bind _newtrack_0 (Timeline|Timeline Play)
      (:Update
        (Transformation|SetWorldRotation (Variables|Default|GetWindow%20Scene) (Math|Rotator|MakeRotator (.roll (Variables|Default|GetWindow%20Rotation)) (.pitch (Variables|Default|GetWindow%20Rotation)) (Math|Float|Lerp (.yaw (Variables|Default|GetWindow%20Rotation)) (+ (.yaw (Variables|Default|GetWindow%20Rotation)) 1.2e+02) _newtrack_0)) false false))
      (:Finished
        (Variables|Default|SetIsLocked false)
        (Rendering|SetVisibility (Variables|/Game/Blueprints/Inventory/BP_Item.BP_Item_C|GetInteractPrompt (Variables|Default|GetAs%20BP%20Item)) true false)))))

(event EventBeginPlay
  (bind _asbp_item (Utilities|Casting|CastToBP_Item (Variables|/Script/Engine.ChildActorComponent|GetChildActor (Variables|Default|GetBP_Item))))
  (bind _output_get (Variables|Default|SetAs%20BP%20Item _asbp_item))
  (Rendering|SetVisibility (Variables|/Game/Blueprints/Inventory/BP_Item.BP_Item_C|GetInteractPrompt _output_get) false false))

(event Collision|EventActorBeginOverlap
  (params (OtherActor :type Actor%20Object%20Reference)))

(event EventTick
  (params (DeltaSeconds :type Float%20%28single-precision%29)))

(fn ConstructionScript
  (Rendering|Components|TextRender|SetText (Variables|Default|GetCodeLabel) (Utilities|Text|ToText(String) (Variables|Default|GetLockerCode))))

(fn InventoryRestricted?
  (return false))

(fn Unlock
  (params (Key%20ID :type String))
  (return false))