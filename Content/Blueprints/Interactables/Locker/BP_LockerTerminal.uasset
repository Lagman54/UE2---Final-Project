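; Interactable keypad terminal that opens whichever BP_Locker in the level matches a three-digit code typed by the player.
; An overlap box shows the use prompt and gates interaction, which switches the view to the terminal, locks and hides the hero and shows the locker HUD.
; Number keys build the code, X clears it, Backspace exits and Enter submits.
; A match on a locked locker blends the camera to it, opens it after a short delay, then restores the player.
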(event OnComponentBeginOverlap(Box)
  (params (OverlappedComponent :type Primitive%20Component%20Object%20Reference) (OtherActor :type Actor%20Object%20Reference) (OtherComp :type Primitive%20Component%20Object%20Reference) (OtherBodyIndex :type Integer) (bFromSweep :type Boolean) (SweepResult :type Hit%20Result%20Structure%20%28by%20ref%29))
  (Utilities|Casting|CastToBP_Hero OtherActor)
  (Rendering|SetVisibility (Variables|Default|GetInteract%20Prompt) true false))

(event OnComponentEndOverlap(Box)
  (params (OverlappedComponent :type Primitive%20Component%20Object%20Reference) (OtherActor :type Actor%20Object%20Reference) (OtherComp :type Primitive%20Component%20Object%20Reference) (OtherBodyIndex :type Integer))
  (Utilities|Casting|CastToBP_Hero OtherActor)
  (Rendering|SetVisibility (Variables|Default|GetInteract%20Prompt) false false))

(event Custom|Open%20Terminal
  (params (Code :type String))
  (Variables|Default|SetAtLeastOneOpened false)
  (bind _array_element (Utilities|Array|ForEachLoopwithBreak (Variables|Default|GetLockers) :!label _label)
    (:LoopBody
      (if (Utilities|Enum|Equal(Enum) Code (Variables|/Game/Blueprints/Interactables/Locker/BP_Locker.BP_Locker_C|GetLockerCode _array_element))
        (if (Variables|/Game/Blueprints/Interactables/Locker/BP_Locker.BP_Locker_C|GetIsLocked _array_element)
          (Variables|Default|Setcurrent%20locker _array_element)
          (Variables|Default|SetAtLeastOneOpened true)
          (goto _label Break)
          (else
            (Development|PrintString "Already opened")))))
    (:Completed
      (if (Variables|Default|GetAtLeastOneOpened)
        (Input|DisableInput (Game|GetPlayerController 0))
        (Development|PrintString "Opening...")
        (Game|Player|SetViewTargetwithBlend (Game|GetPlayerController 0) (Variables|Default|Getcurrent%20locker) 0.0 "VTBlend_Linear" 0.0 false)
        (Utilities|FlowControl|Delay 0.3)
        (Default|Open (Variables|Default|Getcurrent%20locker))
        (Utilities|FlowControl|Delay 2.4)
        (CallFunction|ExitCamera)
        (else
          (Development|PrintString "Invalid code"))))))

(event Custom|NumberEntered
  (params (Number :type String))
  (if (< (Utilities|String|Len (Variables|Default|GetCode%20input)) 3)
    (bind _output_get (Variables|Default|SetCode%20input (Utilities|String|Append (Variables|Default|GetCode%20input) Number)))
    (Rendering|Components|TextRender|SetText (Variables|Default|GetInputCode) (Utilities|Text|ToText(String) _output_get))))

(event Custom|Clear%20input
  (Variables|Default|SetCode%20input "")
  (Rendering|Components|TextRender|SetText (Variables|Default|GetInputCode) (Utilities|Text|MakeLiteralText "- - -")))

(event Custom|Exit%20Camera
  (bind _returnvalue (Game|GetPlayerCharacter 0))
  (bind _interact_prompt (Variables|Default|GetInteract%20Prompt))
  (Game|Player|SetViewTargetwithBlend (Game|GetPlayerController 0) (Game|GetPlayerCharacter 0) 0.0 "VTBlend_Linear" 0.0 false)
  (Input|DisableInput (Game|GetPlayerController 0))
  (bind _asbp_hero (Utilities|Casting|CastToBP_Hero _returnvalue))
  (Default|UnlockCharacter _asbp_hero)
  (Rendering|SetVisibility (Variables|/Script/Engine.Character|GetMesh _returnvalue) true true)
  (Utilities|IsValid _interact_prompt
    (:Is%20Valid
      (Rendering|SetVisibility _interact_prompt true false))
    (:Is%20Not%20Valid
      _))
  (bind _asbp_hero_2 (Utilities|Casting|CastToBP_Hero (Game|GetPlayerCharacter 0)))
  (Default|ShowHUD _asbp_hero_2)
  (Widget|RemovefromParent (Variables|Default|GetWBP%20LockerHUD))
  (CallFunction|ClearInput))

(event EventBeginPlay
  (bind _outactors (Actor|GetAllActorsOfClass "/Game/Blueprints/Interactables/Locker/BP_Locker.BP_Locker_C"))
  (Variables|Default|SetLockers _outactors)
  (bind _aswbp_interact_prompt (Utilities|Casting|CastToWBP_InteractPrompt (UserInterface|GetUserWidgetObject (Variables|Default|GetInteract%20Prompt))))
  (Variables|/Game/UI/WBP_InteractPrompt.WBP_InteractPrompt_C|SetPromptText _aswbp_interact_prompt "[E] Use")
  (Rendering|SetVisibility (Variables|Default|GetInteract%20Prompt) false false)
  (bind _returnvalue (UserInterface|CreateWidget "/Game/Blueprints/Interactables/Locker/WBP_LockerHUD.WBP_LockerHUD_C"))
  (Variables|Default|SetWBP%20LockerHUD _returnvalue))

(event Collision|EventActorBeginOverlap
  (params (OtherActor :type Actor%20Object%20Reference)))

(event EventTick
  (params (DeltaSeconds :type Float%20%28single-precision%29)))

(event EventOnInteract
  (bind _returnvalue (Game|GetPlayerCharacter 0))
  (bind _result (CallFunction|CanInteract))
  (if _result
    (Input|EnableInput (Game|GetPlayerController 0))
    (bind _asbp_hero (Utilities|Casting|CastToBP_Hero _returnvalue))
    (Default|LockCharacter _asbp_hero)
    (Rendering|SetVisibility (Variables|/Script/Engine.Character|GetMesh _returnvalue) false true)
    (Rendering|SetVisibility (Variables|Default|GetInteract%20Prompt) false false)
    (Game|Player|SetViewTargetwithBlend (Game|GetPlayerController 0) self 0.0 "VTBlend_Linear" 0.0 false)
    (bind _asbp_hero_2 (Utilities|Casting|CastToBP_Hero (Game|GetPlayerCharacter 0)))
    (Default|HideHUD _asbp_hero_2)
    (UserInterface|Viewport|AddtoViewport (Variables|Default|GetWBP%20LockerHUD) 0)))

(event Input|KeyboardEvents|1
  (params (Key :type Key%20Structure :default "None"))
  (:Pressed
    (CallFunction|NumberEntered "1")))

(event Input|KeyboardEvents|Backspace
  (params (Key :type Key%20Structure :default "None"))
  (:Pressed
    (CallFunction|ExitCamera)))

(event Input|KeyboardEvents|9
  (params (Key :type Key%20Structure :default "None"))
  (:Pressed
    (CallFunction|NumberEntered "9")))

(event Input|KeyboardEvents|0
  (params (Key :type Key%20Structure :default "None"))
  (:Pressed
    (CallFunction|NumberEntered "0")))

(event Input|KeyboardEvents|X
  (params (Key :type Key%20Structure :default "None"))
  (:Pressed
    (CallFunction|ClearInput)))

(event Input|KeyboardEvents|Enter
  (params (Key :type Key%20Structure :default "None"))
  (bind _code_input (Variables|Default|GetCode%20input))
  (:Pressed
    (if (== (Utilities|String|Len _code_input) 3)
      (CallFunction|OpenTerminal _code_input)
      (CallFunction|ClearInput)
      (else
        (Development|PrintString "code length < 3")))))

(event Input|KeyboardEvents|4
  (params (Key :type Key%20Structure :default "None"))
  (:Pressed
    (CallFunction|NumberEntered "4")))

(event Input|KeyboardEvents|2
  (params (Key :type Key%20Structure :default "None"))
  (:Pressed
    (CallFunction|NumberEntered "2")))

(event Input|KeyboardEvents|3
  (params (Key :type Key%20Structure :default "None"))
  (:Pressed
    (CallFunction|NumberEntered "3")))

(event Input|KeyboardEvents|5
  (params (Key :type Key%20Structure :default "None"))
  (:Pressed
    (CallFunction|NumberEntered "5")))

(event Input|KeyboardEvents|6
  (params (Key :type Key%20Structure :default "None"))
  (:Pressed
    (CallFunction|NumberEntered "6")))

(event Input|KeyboardEvents|7
  (params (Key :type Key%20Structure :default "None"))
  (:Pressed
    (CallFunction|NumberEntered "7")))

(event Input|KeyboardEvents|8
  (params (Key :type Key%20Structure :default "None"))
  (:Pressed
    (CallFunction|NumberEntered "8")))

(fn ConstructionScript)

(fn CanInteract
  (return (Collision|IsOverlappingActor (Variables|Default|GetBox) (Game|GetPlayerCharacter 0) :!class /Script/Engine.PrimitiveComponent)))