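; BP_Window is an interactable window that toggles a close-up camera focus on the hero.
; Its box overlap tracks the hero and swaps the cube's material while they are in range.
; OnInteract, when the hero is in range and not aiming, blocks aiming and plays or reverses a timeline that shortens the spring arm.
; Leaving the box unfocuses automatically, and aiming is allowed again once the zoom-out finishes.
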(event OnComponentEndOverlap(Box)
  (params (OverlappedComponent :type Primitive%20Component%20Object%20Reference) (OtherActor :type Actor%20Object%20Reference) (OtherComp :type Primitive%20Component%20Object%20Reference) (OtherBodyIndex :type Integer))
  (Utilities|Casting|CastToBP_Hero OtherActor)
  (Variables|Default|SetOverlapsCharacter false)
  (Rendering|Material|SetMaterial (Variables|Default|GetCube) 0 "/Engine/BasicShapes/BasicShapeMaterial.BasicShapeMaterial")
  (if (Variables|Default|GetIsFocused)
    (CallFunction|UnfocusWindow)))

(event OnComponentBeginOverlap(Box)
  (params (OverlappedComponent :type Primitive%20Component%20Object%20Reference) (OtherActor :type Actor%20Object%20Reference) (OtherComp :type Primitive%20Component%20Object%20Reference) (OtherBodyIndex :type Integer) (bFromSweep :type Boolean) (SweepResult :type Hit%20Result%20Structure%20%28by%20ref%29))
  (Utilities|Casting|CastToBP_Hero OtherActor)
  (Variables|Default|SetOverlapsCharacter true)
  (Rendering|Material|SetMaterial (Variables|Default|GetCube) 0 "/Engine/MapTemplates/Materials/BasicAsset03.BasicAsset03"))

(event Custom|Focus%20Window
  ;[0.15 0.15 0.15 0.5] Focus window
  (if (not (Variables|/Game/Character/BP_Hero.BP_Hero_C|GetIsAiming (Variables|Default|GetAs%20BP%20Hero)))
    (bind _result (CallFunction|IsOverlapping))
    (if _result
      (Variables|/Game/Character/BP_Hero.BP_Hero_C|SetAimingAllowed (Variables|Default|GetAs%20BP%20Hero) false)
      (if (Variables|Default|GetIsFocused)
        (Variables|Default|SetIsFocused false)
        (bind _newtrack_0 (Timeline|Timeline Reverse)
          (:Update
            (Variables|/Script/Engine.SpringArmComponent|SetTargetArmLength (Variables|/Game/Character/BP_Hero.BP_Hero_C|GetSpringArm (Variables|Default|GetAs%20BP%20Hero)) (Math|Float|Lerp 2e+02 1e+02 _newtrack_0)))
          (:Finished
            (if (Variables|Default|GetIsFocused)
              (Variables|/Game/Character/BP_Hero.BP_Hero_C|SetAimingAllowed (Variables|Default|GetAs%20BP%20Hero) false)
              (else
                (Variables|/Game/Character/BP_Hero.BP_Hero_C|SetAimingAllowed (Variables|Default|GetAs%20BP%20Hero) true)))))
        (else
          (Variables|Default|SetIsFocused true)
          (Timeline|Timeline PlayFromStart))))))

(event Custom|Unfocus%20Window
  ;[0.15 0.15 0.15 0.5] Focus window
  (Variables|/Game/Character/BP_Hero.BP_Hero_C|SetAimingAllowed (Variables|Default|GetAs%20BP%20Hero) false)
  (if (Variables|Default|GetIsFocused)
    (Variables|Default|SetIsFocused false)
    (bind _newtrack_0 (Timeline|Timeline Reverse)
      (:Update
        (Variables|/Script/Engine.SpringArmComponent|SetTargetArmLength (Variables|/Game/Character/BP_Hero.BP_Hero_C|GetSpringArm (Variables|Default|GetAs%20BP%20Hero)) (Math|Float|Lerp 2e+02 1e+02 _newtrack_0)))
      (:Finished
        (if (Variables|Default|GetIsFocused)
          (Variables|/Game/Character/BP_Hero.BP_Hero_C|SetAimingAllowed (Variables|Default|GetAs%20BP%20Hero) false)
          (else
            (Variables|/Game/Character/BP_Hero.BP_Hero_C|SetAimingAllowed (Variables|Default|GetAs%20BP%20Hero) true)))))
    (else
      (Variables|Default|SetIsFocused true)
      (Timeline|Timeline PlayFromStart))))

(event EventBeginPlay
  (bind _asbp_hero (Utilities|Casting|CastToBP_Hero (Game|GetPlayerCharacter 0)))
  (Variables|Default|SetAs%20BP%20Hero _asbp_hero))

(event Collision|EventActorBeginOverlap
  (params (OtherActor :type Actor%20Object%20Reference)))

(event EventTick
  (params (DeltaSeconds :type Float%20%28single-precision%29)))

(event EventOnInteract
  (CallFunction|FocusWindow))

(fn ConstructionScript)

(fn Interact)

(fn IsOverlapping
  (return (Variables|Default|GetOverlapsCharacter)))

(fn CanInteract
  (return false))